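; Base grid creature for a turn-based game, with movement, pickup, attack, damage and death, plus an info visualiser shown on cursor hover.
; Moves and attacks spend substeps; movement offsets the actor by Procedual's PolygonSize and updates cell occupancy on MyActor.
; Pickup and attack match grid positions against TurnBased's arrays, returning after the first element.
; Damage subtracts BaseDefense and triggers Die, while Heal adds zero and UseItem is empty.
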(event EventBeginPlay
  ;[1 1 1] Initial assignments
)

(event Collision|EventActorBeginOverlap
  (params (OtherActor :type Actor%20Object%20Reference)))

(event EventTick
  (params (DeltaSeconds :type Float%20%28single-precision%29)))

(event MouseInput|EventActorBeginCursorOver
  (Default|On (Variables|Default|GetInfoVisualiser)))

(event MouseInput|EventActorEndCursorOver
  (Default|Off (Variables|Default|GetInfoVisualiser)))

(event EventDestroyed
  (Default|Off (Variables|Default|GetInfoVisualiser)))

(fn ConstructionScript)

(fn TryMove
  (params (To%20Move :type Int%20Vector%20Structure))
  (bind (_x _y) (Utilities|Struct|BreakIntVector To%20Move))
  (bind (_x_2 _y_2) (Utilities|Struct|BreakIntVector To%20Move))
  (bind _returnvalue (Actor|GetActorOfClass "/Game/Blueprints/PROCEDUAL.Procedual_C"))
  (bind _returnvalue_2 (Actor|GetActorOfClass "/Script/Prototype.MyActor"))
  (if (Class|MyActor|CheckifBlocked _returnvalue_2 (Utilities|Struct|MakeIntVector (+ _x (.X (Utilities|Struct|BreakIntVector (Variables|BattleCharacteristics|GetPosition)))) (+ _y (.Y (Utilities|Struct|BreakIntVector (Variables|BattleCharacteristics|GetPosition))))))
    (Transformation|AddActorLocalOffset (Math|Vector|MakeVector (* _x_2 (Math|Conversions|ToFloat(Integer) (Variables|/Game/Blueprints/PROCEDUAL.Procedual_C|GetPolygon%20Size _returnvalue))) (* _y_2 (Math|Conversions|ToFloat(Integer) (Variables|/Game/Blueprints/PROCEDUAL.Procedual_C|GetPolygon%20Size _returnvalue))) 0.0) false false)
    (Class|MyActor|SetCellIsOccupied _returnvalue_2 (.x (Variables|BattleCharacteristics|GetPosition)) (.y (Variables|BattleCharacteristics|GetPosition)))
    (bind _output_get (Variables|BattleCharacteristics|SetPosition (Utilities|Struct|MakeIntVector (+ _x (.X (Utilities|Struct|BreakIntVector (Variables|BattleCharacteristics|GetPosition)))) (+ _y (.Y (Utilities|Struct|BreakIntVector (Variables|BattleCharacteristics|GetPosition)))))))
    (Class|MyActor|SetCellIsOccupied _returnvalue_2 (.x _output_get) (.y _output_get) 2)
    (Math|Integer|DecrementInt (Variables|BattleCharacteristics|GetNumber%20Of%20Remaining%20Substeps)
      (:%20%20
        (return true)))
    (else
      (return false))))

(fn TryPickUp
  (bind _position (Variables|BattleCharacteristics|GetPosition))
  (bind (_x _y) (Utilities|Struct|BreakIntVector _position))
  (bind _returnvalue (Actor|GetActorOfClass "/Game/Blueprints/Turn-Based.Turn-Based_C"))
  (bind _array_element (Utilities|Array|ForEachLoopwithBreak (Variables|/Game/Blueprints/Turn-Based.Turn-Based_C|GetArrayOfPickUps _returnvalue))
    (:LoopBody
      (if (and (== (.X (Utilities|Struct|BreakIntVector (Variables|/Game/Blueprints/PickUp.PickUp_C|GetPosition _array_element))) _x) (== (.Y (Utilities|Struct|BreakIntVector (Variables|/Game/Blueprints/PickUp.PickUp_C|GetPosition _array_element))) _y))
        (Default|PickUp _array_element)
        (return true)
        (else
          (return false))))))

(fn ReceiveDamageBase
  (params (Damage :type Integer))
  (bind _basedefense (Variables|BattleCharacteristics|GetbaseDefense))
  (bind _returnvalue (- Damage _basedefense))
  (if (> _returnvalue 0)
    (bind _output_get (Variables|BattleCharacteristics|SetHP (- (Variables|BattleCharacteristics|GetHP) _returnvalue)))
    (if (<= _output_get 0)
      (return true)
      (else
        (return false)))))

(fn TryAttack
  (params (Where :type Int%20Vector%20Structure%20%28by%20ref%29))
  (bind (_x _y) (Utilities|Struct|BreakIntVector Where))
  (bind _position (Variables|BattleCharacteristics|GetPosition))
  (bind (_x_2 _y_2) (Utilities|Struct|BreakIntVector _position))
  (bind _returnvalue (Actor|GetActorOfClass "/Game/Blueprints/Turn-Based.Turn-Based_C"))
  (bind _array_element (Utilities|Array|ForEachLoopwithBreak (Variables|/Game/Blueprints/Turn-Based.Turn-Based_C|GetArrayOfNPCs _returnvalue))
    (:LoopBody
      (if (and (== (.X (Utilities|Struct|BreakIntVector (Variables|Creature_C|GetPosition _array_element))) (+ _x _x_2)) (== (.Y (Utilities|Struct|BreakIntVector (Variables|Creature_C|GetPosition _array_element))) (+ _y _y_2)))
        (Development|PrintString "Attacking!")
        (Variables|BattleCharacteristics|SetIs%20in%20combat true)
        (bind _asnpc (Utilities|Casting|CastToNPC _array_element))
        (if (Variables|Creature_C|GetIs%20in%20combat _array_element)
          (Default|ReceiveDamage0 _asnpc (Variables|BattleCharacteristics|GetbaseAttack) self)
          (else
            (Default|ReceiveDamage0 _asnpc 0 self)))
        (Math|Integer|DecrementInt (Variables|BattleCharacteristics|GetNumber%20Of%20Remaining%20Substeps)
          (:%20%20
            (return true)))
        (else
          (return false))))))

(fn Die
  (bind _position (Variables|BattleCharacteristics|GetPosition))
  (bind (_x _y) (Utilities|Struct|BreakIntVector _position))
  (bind _returnvalue (Actor|GetActorOfClass "/Script/Prototype.MyActor"))
  (Development|PrintString "Died" true true "(R=1.000000,G=0.043376,B=0.000000,A=1.000000)")
  (Class|MyActor|SetCellIsOccupied _returnvalue _x _y)
  (Actor|DestroyActor))

(fn Heal
  (bind _maxhp (Variables|BattleCharacteristics|GetmaxHP))
  (if (<= (+ 0 (Variables|BattleCharacteristics|GetHP)) _maxhp)
    (Variables|BattleCharacteristics|SetHP (+ 0 (Variables|BattleCharacteristics|GetHP)))
    (else
      (Variables|BattleCharacteristics|SetHP _maxhp))))

(fn ReceiveDamage
  (params (Damage :type Integer))
  (bind _diddie (CallFunction|ReceiveDamageBase Damage))
  (if _diddie
    (CallFunction|Die)
    (return true)
    (else
      (return false))))

(fn UseItem)