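; Turn-based lava hazard actor that spreads by Game of Life rules, acting as its own participant in the turn order.
; Each turn it steps the simulation with editable birth/survive rules (Conway's by default) and updates lava pieces on the field.
; It redraws the cells to a dynamic canvas texture on Plane1's material.
; Creatures on live cells take damage, a Flash sequence plays, and after a short delay TurnBased advances.
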(event Custom|End%20Turn
  (bind _returnvalue (Actor|GetActorOfClass "/Game/Blueprints/Turn-Based.Turn-Based_C"))
  (Default|NextTurn _returnvalue))

(event EventBeginPlay
  ;[1 1 1] drawing in dynamic texture
  (bind _returnvalue (Game|ConstructObjectfromClass "/Script/Prototype.DrawingCanvas" self))
  (Variables|Default|Setcanvas _returnvalue)
  (bind _returnvalue_2 (Rendering|Material|CreateDynamicMaterialInstance (Variables|Default|GetPlane1) 0 "/Game/test.test" "None" :!class /Script/Engine.PrimitiveComponent))
  (Variables|Default|SetMatInst _returnvalue_2)
  (Class|DrawingCanvas|InitializeCanvas (Variables|Default|Getcanvas) 256 256)
  (Rendering|Material|SetTextureParameterValue (Variables|Default|GetMatInst) "InputTexture" (Variables|/Script/Prototype.DrawingCanvas|GetdynamicCanvas (Variables|Default|Getcanvas)))
  (Class|DrawingCanvas|DrawLife (Variables|Default|Getcanvas) self)
  (Rendering|Material|SetTextureParameterValue (Variables|Default|GetMatInst) "InputTexture" (Variables|/Script/Prototype.DrawingCanvas|GetdynamicCanvas (Variables|Default|Getcanvas))))

(event Collision|EventActorBeginOverlap
  (params (OtherActor :type Actor%20Object%20Reference)))

(event EventStartTurn
  (bind _canvas (Variables|Default|Getcanvas))
  (CallFunction|MessagetoList "Lava" "'s turn" " ")
  ;[1 1 1] GoL Update
  (bind _returnvalue (Actor|GetActorOfClass "/Game/Blueprints/PROCEDUAL.Procedual_C"))
  (bind _returnvalue_2 (Actor|GetActorOfClass "/Script/Prototype.MyActor"))
  ;;[1 1 1] Here is a place where you can change birth and survive value. You can put here loops, if-branches, randomizers and anything else you want
  (bind _output_get (Variables|/Game/Blueprints/PROCEDUAL.Procedual_C|Setbirth _returnvalue (Utilities|Array|MakeArray false false false true false false false false false)))
  (bind _output_get_2 (Variables|/Game/Blueprints/PROCEDUAL.Procedual_C|Setsurvive _returnvalue (Utilities|Array|MakeArray false false true true false false false false false)))
  (Class|GoLUser|UpdateGoL _output_get _output_get_2 _returnvalue_2 3 true)
  (bind _returnvalue_3 (Class|GoLUser|UpdateLavaPiecesonField (Variables|/Game/Blueprints/PROCEDUAL.Procedual_C|GetPolygon%20Size _returnvalue)))
  (Utilities|FlowControl|Sequence
    (:then_0
      ;[1 1 1] drawing in dynamic texture
      (Class|DrawingCanvas|ClearCanvas _canvas)
      (Class|DrawingCanvas|DrawLife _canvas self)
      (Rendering|Material|SetTextureParameterValue (Variables|Default|GetMatInst) "InputTexture" (Variables|/Script/Prototype.DrawingCanvas|GetdynamicCanvas (Variables|Default|Getcanvas))))
    (:then_1
      ;[1 1 1] Lit creatures on fire
      (bind _outactors (Actor|GetAllActorsOfClass "/Game/Blueprints/Creature.Creature_C"))
      (for _array_element _outactors
        (if (Class|GoLUser|IsAlive (.x (Variables|/Game/Blueprints/Creature.Creature_C|GetPosition _array_element)) (.y (Variables|/Game/Blueprints/Creature.Creature_C|GetPosition _array_element)))
          (Default|ReceiveDamage _array_element 6 1)))
      (Utilities|FlowControl|Sequence
        (:then_0
          (Utilities|FlowControl|Delay 1.0)
          (CallFunction|EndTurn))
        (:then_1
          (bind _returnvalue_4 (Sequencer|Player|CreateLevelSequencePlayer "/Game/Flash.Flash"))
          (Sequencer|Player|Play _returnvalue_4 :!class /Script/MovieScene.MovieSceneSequencePlayer))))))

(fn ConstructionScript)