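; Level builder that turns MyActor's generated grid into a playable turn-based map on BeginPlay.
; FLOORGENERATOR builds vertices, triangles and tiled UVs for a collidable procedural mesh floor, then border walls and Blocks for occupied cells are spawned.
; It places the PlayerPawn at the start, a glass Block at the finish and NPCs at enemy positions.
; Cell occupancy codes are written back to MyActor, while obstacle Blocks and NPCs register with TurnBased.
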(event EventBeginPlay
  (bind _proceduralmesh (Variables|Default|GetProceduralMesh))
  (bind _returnvalue (Actor|GetActorOfClass "/Script/Prototype.MyActor"))
  ;[1 1 1] Consts
  (Variables|Default|SetPolygon%20Size 100)
  (Utilities|FlowControl|Sequence
    (:then_0
      ;;[1 1 1] Generation of level
      (Class|MyActor|GenerateLevel _returnvalue 32 32))
    (:then_1
      ;[1 1 1] Creation of floor
      (bind _returnvalue_2 (Class|MyActor|GetHeight _returnvalue))
      (bind _returnvalue_3 (Class|MyActor|GetWidth _returnvalue))
      (bind _output_get (Variables|Default|SetUV%20Scale (Math|Conversions|ToFloat(Integer) (* _returnvalue_2 _returnvalue_3))))
      (CallFunction|FLOORGENERATOR (Variables|Default|GetPolygon%20Size) (+ _returnvalue_2 1) (+ _returnvalue_3 1) _output_get)
      (Class|ProceduralMeshComponent|CreateMeshSectionLinearColor _proceduralmesh 0 (Variables|Default|GetVERTICES) (Variables|Default|GetTRIANGLES) 0 (Variables|Default|GetUV) 0 0 0 0 0 true)
      (Rendering|Material|SetMaterial _proceduralmesh 0 "/Game/StarterContent/Materials/M_CobbleStone_Pebble.M_CobbleStone_Pebble"))
    (:then_2
      ;[1 1 1] Creation of blocks
      (bind _returnvalue_4 (Actor|GetActorOfClass "/Game/Blueprints/Turn-Based.Turn-Based_C"))
      (for _index (range 0 (- _returnvalue_2 1))
        (for _index_2 (range 0 (- _returnvalue_3 1))
          (bind _returnvalue_5 (Class|MyActor|GetCellIsOccupied _returnvalue _index _index_2))
          (if (== _returnvalue_5 1)
            (bind _returnvalue_6 (Game|SpawnActorfromClass "/Game/Blueprints/Block.Block_C" (Math|Transform|MakeTransform (Math|Vector|MakeVector (* (+ (Math|Conversions|ToFloat(Integer) _index) 0.5) (Math|Conversions|ToFloat(Integer) (Variables|Default|GetPolygon%20Size))) (* (Math|Conversions|ToFloat(Integer) (Variables|Default|GetPolygon%20Size)) (+ (Math|Conversions|ToFloat(Integer) _index_2) 0.5)) 5e+01) "0, 0, 0" "1,1,1") "Undefined" 0 (Utilities|Struct|MakeIntVector _index _index_2 0) 0))
            (Class|MyActor|SetCellIsOccupied _returnvalue _index _index_2 1)
            (Rendering|Material|SetMaterial (Variables|/Game/Blueprints/Block.Block_C|GetCube _returnvalue_6) 0 "/Game/StarterContent/Materials/M_Brick_Clay_New.M_Brick_Clay_New")
            (Utilities|Array|Add (Variables|/Game/Blueprints/Turn-Based.Turn-Based_C|GetArrayOfBlocks _returnvalue_4) _returnvalue_6)
            (else
              (Class|MyActor|SetCellIsOccupied _returnvalue _index _index_2))))))
    (:then_3
      ;[1 1 1] Creation of Walls
      (Utilities|FlowControl|Sequence
        (:then_0
          (for _index_3 (range 0 (- _returnvalue_2 1))
            (bind _returnvalue_7 (Game|SpawnActorfromClass "/Script/Engine.StaticMeshActor" (Math|Transform|MakeTransform (Math|Vector|MakeVector (* (Math|Conversions|ToFloat(Integer) _index_3) (Math|Conversions|ToFloat(Integer) (Variables|Default|GetPolygon%20Size))) 0.0 0.0) "0, 0, 0" "0.250000,1.000000,5.000000") "Undefined" 0 0))
            (Components|StaticMesh|SetStaticMesh (Variables|/Script/Engine.StaticMeshActor|GetStaticMeshComponent _returnvalue_7) "/Game/StarterContent/Architecture/Wall_400x400.Wall_400x400")
            (Rendering|Material|SetMaterial (Variables|/Script/Engine.StaticMeshActor|GetStaticMeshComponent _returnvalue_7) 0 "/Game/StarterContent/Materials/M_Wood_Pine.M_Wood_Pine")
            (bind _returnvalue_8 (Game|SpawnActorfromClass "/Script/Engine.StaticMeshActor" (Math|Transform|MakeTransform (Math|Vector|MakeVector (* (Math|Conversions|ToFloat(Integer) _index_3) (Math|Conversions|ToFloat(Integer) (Variables|Default|GetPolygon%20Size))) (* (Math|Conversions|ToFloat(Integer) (Variables|Default|GetPolygon%20Size)) (Math|Conversions|ToFloat(Integer) (+ (- _returnvalue_3 1) 1))) 0.0) "0, 0, 0" "0.250000,1.000000,5.000000") "Undefined" 0 0))
            (Components|StaticMesh|SetStaticMesh (Variables|/Script/Engine.StaticMeshActor|GetStaticMeshComponent _returnvalue_8) "/Game/StarterContent/Architecture/Wall_400x400.Wall_400x400")
            (Rendering|Material|SetMaterial (Variables|/Script/Engine.StaticMeshActor|GetStaticMeshComponent _returnvalue_8) 0 "/Game/StarterContent/Materials/M_Wood_Pine.M_Wood_Pine")))
        (:then_1
          (for _index_4 (range 0 (- _returnvalue_3 1))
            (bind _returnvalue_9 (Game|SpawnActorfromClass "/Script/Engine.StaticMeshActor" (Math|Transform|MakeTransform (Math|Vector|MakeVector 0.0 (* (Math|Conversions|ToFloat(Integer) _index_4) (Math|Conversions|ToFloat(Integer) (Variables|Default|GetPolygon%20Size))) 0.0) "0,90.000000, 0" "0.250000,1.000000,5.000000") "Undefined" 0 0))
            (Components|StaticMesh|SetStaticMesh (Variables|/Script/Engine.StaticMeshActor|GetStaticMeshComponent _returnvalue_9) "/Game/StarterContent/Architecture/Wall_400x400.Wall_400x400")
            (Rendering|Material|SetMaterial (Variables|/Script/Engine.StaticMeshActor|GetStaticMeshComponent _returnvalue_9) 0 "/Game/StarterContent/Materials/M_Wood_Pine.M_Wood_Pine")
            (bind _returnvalue_10 (Game|SpawnActorfromClass "/Script/Engine.StaticMeshActor" (Math|Transform|MakeTransform (Math|Vector|MakeVector (* (Math|Conversions|ToFloat(Integer) (Variables|Default|GetPolygon%20Size)) (Math|Conversions|ToFloat(Integer) (+ (- _returnvalue_2 1) 1))) (* (Math|Conversions|ToFloat(Integer) _index_4) (Math|Conversions|ToFloat(Integer) (Variables|Default|GetPolygon%20Size))) 0.0) "0,90.000000, 0" "0.250000,1.000000,5.000000") "Undefined" 0 0))
            (Components|StaticMesh|SetStaticMesh (Variables|/Script/Engine.StaticMeshActor|GetStaticMeshComponent _returnvalue_10) "/Game/StarterContent/Architecture/Wall_400x400.Wall_400x400")
            (Rendering|Material|SetMaterial (Variables|/Script/Engine.StaticMeshActor|GetStaticMeshComponent _returnvalue_10) 0 "/Game/StarterContent/Materials/M_Wood_Pine.M_Wood_Pine")))))
    (:then_4
      ;[1 1 1] Creation of start and finish
      (Utilities|FlowControl|Sequence
        (:then_0
          (bind _returnvalue_11 (Class|MyActor|GetStartPosition _returnvalue))
          (bind _returnvalue_12 (Actor|GetActorOfClass "/Game/Blueprints/PlayerPawn.PlayerPawn_C"))
          (Transformation|SetActorLocation _returnvalue_12 (* (+ _returnvalue_11 "0.500000,0.500000,1.000000") (Math|Conversions|ToFloat(Integer) (Variables|Default|GetPolygon%20Size))) false false)
          (bind _output_get_2 (Variables|/Game/Blueprints/Creature.Creature_C|SetPosition _returnvalue_12 (Class|KismetMathLibrary|FTruncVector _returnvalue_11)))
          (Class|MyActor|SetCellIsOccupied _returnvalue (.x _output_get_2) (.y _output_get_2) 3))
        (:then_1
          (bind _returnvalue_13 (Class|MyActor|GetFinishPosition _returnvalue))
          (bind _returnvalue_14 (Game|SpawnActorfromClass "/Game/Blueprints/Block.Block_C" (Math|Transform|MakeTransform (* (+ _returnvalue_13 "0.500000,0.500000,1.000000") (Math|Conversions|ToFloat(Integer) (Variables|Default|GetPolygon%20Size))) "0, 0, 0" "1,1,1") "Undefined" 0 (Class|KismetMathLibrary|FTruncVector _returnvalue_13) 0))
          (Components|StaticMesh|SetStaticMesh (Variables|/Game/Blueprints/Block.Block_C|GetCube _returnvalue_14) "/Engine/Functions/Engine_MaterialFunctions02/ExampleContent/PivotPainter2/SimplePivotPainterExample.SimplePivotPainterExample")
          (Rendering|Material|SetMaterial (Variables|/Game/Blueprints/Block.Block_C|GetCube _returnvalue_14) 0 "/DatasmithContent/Materials/FBXImporter/VRED/Glass.Glass")
          (Class|MyActor|SetCellIsOccupied _returnvalue (.x (Variables|/Game/Blueprints/Block.Block_C|GetPosition _returnvalue_14)) (.y (Variables|/Game/Blueprints/Block.Block_C|GetPosition _returnvalue_14)) 4))))
    (:then_5
      ;[1 1 1] Creation of NPCs
      (bind _returnvalue_15 (Class|MyActor|GetNumberOfEnemies _returnvalue))
      (for _index_5 (range 0 (- _returnvalue_15 1))
        (bind _returnvalue_16 (Class|MyActor|GetEnemyPosition _returnvalue _index_5))
        (bind _returnvalue_17 (Game|SpawnActorfromClass "/Game/Blueprints/NPC.NPC_C" (Math|Transform|MakeTransform (* (+ _returnvalue_16 "0.500000,0.500000,1.000000") (Math|Conversions|ToFloat(Integer) (Variables|Default|GetPolygon%20Size))) "0, 0, 0" "1,1,1") "Undefined" 0 0))
        (bind _output_get_3 (Variables|/Game/Blueprints/Creature.Creature_C|SetPosition _returnvalue_17 (Class|KismetMathLibrary|FTruncVector _returnvalue_16)))
        (bind _returnvalue_18 (Actor|GetActorOfClass "/Game/Blueprints/Turn-Based.Turn-Based_C"))
        (Class|MyActor|SetCellIsOccupied _returnvalue (.x _output_get_3) (.y _output_get_3) 2)
        (Utilities|Array|Add (Variables|/Game/Blueprints/Turn-Based.Turn-Based_C|GetArrayOfNPCs _returnvalue_18) _returnvalue_17)))))

(event EventTick
  (params (DeltaSeconds :type Float%20%28single-precision%29)))

(event Collision|EventActorBeginOverlap
  (params (OtherActor :type Actor%20Object%20Reference)))

(fn ConstructionScript)

(fn FLOORGENERATOR
  (params (Polygon%20size :type Integer) (Height :type Integer) (WIdth :type Integer) (UV%20Scale :type Float%20%28single-precision%29))
  (bind _returnvalue (- WIdth 1))
  (bind _returnvalue_2 (- Height 1))
  (Utilities|Array|Clear (Variables|Default|GetVERTICES))
  (Utilities|Array|Clear (Variables|Default|GetTRIANGLES))
  (for _index (range 0 _returnvalue_2)
    (for _index_2 (range 0 _returnvalue)
      (Utilities|FlowControl|Sequence
        (:then_0
          ;[1 1 1] Vertices
          (Utilities|Array|Add (Variables|Default|GetVERTICES) (Math|Vector|MakeVector (Math|Conversions|ToFloat(Integer) (* _index Polygon%20size)) (Math|Conversions|ToFloat(Integer) (* _index_2 Polygon%20size)) 0.0)))
        (:then_1
          ;[1 1 1] Triangles
          (if (and (!= _index _returnvalue_2) (!= _index_2 _returnvalue))
            (Class|KismetProceduralMeshLibrary|ConvertQuadtoTriangles (Variables|Default|GetTRIANGLES) (+ _index_2 (* _index WIdth)) (+ (+ _index_2 (* _index WIdth)) 1) (+ (+ _index_2 (* (+ _index 1) WIdth)) 1) (+ _index_2 (* (+ _index 1) WIdth)))))
        (:then_2
          ;[1 1 1] UV
          (Utilities|Array|Add (Variables|Default|GetUV) (Math|Vector2D|MakeVector2D (* (/ 1.0 (Math|Conversions|ToFloat(Integer) _returnvalue_2)) (Math|Conversions|ToFloat(Integer) _index) UV%20Scale) (* UV%20Scale (Math|Conversions|ToFloat(Integer) _index_2) (/ 1.0 (Math|Conversions|ToFloat(Integer) _returnvalue))))))))))