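; Level builder actor that, on BeginPlay, constructs a grid-based level in tutorial or generated mode, sized from the Global game instance.
; MyActor generates and holds the grid, which drives a procedural floor mesh, border walls, blocks, finish marker, player placement and NPC spawns.
; Spawning writes cell occupancy back to MyActor and registers position-list blocks with TurnBased.
; GoLUser runs Game of Life iterations on the grid to lay out lava.
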(event EventBeginPlay
  (bind _proceduralmesh (Variables|Default|GetProceduralMesh))
  (bind _tutor (Variables|Default|GetTutor))
  (bind _returnvalue (Actor|GetActorOfClass "/Script/Prototype.MyActor"))
  (bind _asglobal (Utilities|Casting|CastToGlobal (Game|GetGameInstance)))
  (Utilities|FlowControl|Sequence
    (:then_0
      (Variables|Default|SetPolygon%20Size 100)
      (if (Variables|Default|GetTutor)
        (Class|MyActor|GenerateTutor _returnvalue 5 15)
        (else
          ;[1 1 1] Consts
          ;;[1 1 1] Generation of level
          (Class|MyActor|GenerateLevel _returnvalue (Variables|/Game/Blueprints/Global.Global_C|GetGHeight _asglobal) (Variables|/Game/Blueprints/Global.Global_C|GetGWidth _asglobal)))))
    (:then_1
      ;[1 1 1] Creation of floor
      (bind _output_get (Variables|Default|SetUV%20Scale (* (Math|Conversions|ToFloat(Integer) (* (Class|MyActor|GetHeight _returnvalue) (Class|MyActor|GetWidth _returnvalue))) 0.025)))
      (CallFunction|FLOORGENERATOR (Variables|Default|GetPolygon%20Size) (+ (Class|MyActor|GetHeight _returnvalue) 1) (+ (Class|MyActor|GetWidth _returnvalue) 1) _output_get)
      (Class|ProceduralMeshComponent|CreateMeshSectionLinearColor _proceduralmesh 0 (Variables|Default|GetVERTICES) (Variables|Default|GetTRIANGLES) 0 (Variables|Default|GetUV) 0 0 0 0 0 true)
      (Rendering|Material|SetMaterial _proceduralmesh 0 "/Game/StarterContent/Materials/M_Concrete_Grime.M_Concrete_Grime"))
    (:then_2
      ;[1 1 1] Creation of map
      (for _index (range 0 (- (Class|MyActor|GetHeight _returnvalue) 1))
        (for _index_2 (range 0 (- (Class|MyActor|GetWidth _returnvalue) 1))
          (if (== (Class|MyActor|GetCellIsOccupied _returnvalue _index _index_2) 1)
            (bind _returnvalue_2 (Game|SpawnActorfromClass "/Game/Blueprints/Block.Block_C" (Math|Transform|MakeTransform (Math|Vector|MakeVector (* (+ (Math|Conversions|ToFloat(Integer) _index) 0.5) (Math|Conversions|ToFloat(Integer) (Variables|Default|GetPolygon%20Size))) (* (Math|Conversions|ToFloat(Integer) (Variables|Default|GetPolygon%20Size)) (+ (Math|Conversions|ToFloat(Integer) _index_2) 0.5)) 5e+01) "0, 0, 0" "1,1,1") "Undefined" 0 (Utilities|Struct|MakeIntVector _index _index_2 0) 0))
            (Class|MyActor|SetCellIsOccupied _returnvalue _index _index_2 1)
            (Rendering|Material|SetMaterial (Variables|/Game/Blueprints/Block.Block_C|GetCube _returnvalue_2) 0 "/Game/StarterContent/Materials/M_Brick_Clay_New.M_Brick_Clay_New")
            (else
              (Class|MyActor|SetCellIsOccupied _returnvalue _index _index_2))))))
    (:then_3
      ;[1 1 1] Creation of blocks
      (for _index_3 (range 0 (- (Class|MyActor|GetNumberOfBlocks _returnvalue) 1))
        (bind _returnvalue_3 (Game|SpawnActorfromClass :Class "/Game/Blueprints/Block.Block_C" :SpawnTransform (Math|Transform|MakeTransform (* (+ (Math|Conversions|ToVector(Float) (Class|MyActor|GetBlockPosition _returnvalue _index_3)) "0.500000,0.500000,1.000000") (Math|Conversions|ToFloat(Integer) (Variables|Default|GetPolygon%20Size))) "0, 0, 0" "1,1,1") :CollisionHandlingOverride "Undefined" :Instigator 0))
        (bind _output_get_2 (Variables|/Game/Blueprints/Block.Block_C|SetPosition _returnvalue_3 (Class|MyActor|GetBlockPosition _returnvalue _index_3)))
        (bind _returnvalue_4 (Actor|GetActorOfClass "/Game/Blueprints/Turn-Based.Turn-Based_C"))
        (Class|MyActor|SetCellIsOccupied _returnvalue (.x _output_get_2) (.y _output_get_2) 3)
        (Utilities|Array|Add (Variables|/Game/Blueprints/Turn-Based.Turn-Based_C|GetArrayOfBlocks _returnvalue_4) _returnvalue_3)))
    (:then_4
      ;[1 1 1] Creation of Walls
      (Utilities|FlowControl|Sequence
        (:then_0
          (for _index_4 (range 0 (- (Class|MyActor|GetHeight _returnvalue) 1))
            (bind _returnvalue_5 (Game|SpawnActorfromClass "/Script/Engine.StaticMeshActor" (Math|Transform|MakeTransform (Math|Vector|MakeVector (* (Math|Conversions|ToFloat(Integer) _index_4) (Math|Conversions|ToFloat(Integer) (Variables|Default|GetPolygon%20Size))) 0.0 0.0) "0, 0, 0" "0.250000,1.000000,5.000000") "Undefined" 0 0))
            (Components|StaticMesh|SetStaticMesh (Variables|/Script/Engine.StaticMeshActor|GetStaticMeshComponent _returnvalue_5) "/Game/StarterContent/Architecture/Wall_400x400.Wall_400x400")
            (Rendering|Material|SetMaterial (Variables|/Script/Engine.StaticMeshActor|GetStaticMeshComponent _returnvalue_5) 0 "/Game/StarterContent/Materials/M_Wood_Pine.M_Wood_Pine")
            (bind _returnvalue_6 (Game|SpawnActorfromClass "/Script/Engine.StaticMeshActor" (Math|Transform|MakeTransform (Math|Vector|MakeVector (* (Math|Conversions|ToFloat(Integer) _index_4) (Math|Conversions|ToFloat(Integer) (Variables|Default|GetPolygon%20Size))) (* (Math|Conversions|ToFloat(Integer) (Variables|Default|GetPolygon%20Size)) (Math|Conversions|ToFloat(Integer) (+ (- (Class|MyActor|GetWidth _returnvalue) 1) 1))) 0.0) "0, 0, 0" "0.250000,1.000000,5.000000") "Undefined" 0 0))
            (Components|StaticMesh|SetStaticMesh (Variables|/Script/Engine.StaticMeshActor|GetStaticMeshComponent _returnvalue_6) "/Game/StarterContent/Architecture/Wall_400x400.Wall_400x400")
            (Rendering|Material|SetMaterial (Variables|/Script/Engine.StaticMeshActor|GetStaticMeshComponent _returnvalue_6) 0 "/Game/StarterContent/Materials/M_Wood_Pine.M_Wood_Pine")))
        (:then_1
          (for _index_5 (range 0 (- (Class|MyActor|GetWidth _returnvalue) 1))
            (bind _returnvalue_7 (Game|SpawnActorfromClass "/Script/Engine.StaticMeshActor" (Math|Transform|MakeTransform (Math|Vector|MakeVector 0.0 (* (Math|Conversions|ToFloat(Integer) _index_5) (Math|Conversions|ToFloat(Integer) (Variables|Default|GetPolygon%20Size))) 0.0) "0,90.000000, 0" "0.250000,1.000000,5.000000") "Undefined" 0 0))
            (Components|StaticMesh|SetStaticMesh (Variables|/Script/Engine.StaticMeshActor|GetStaticMeshComponent _returnvalue_7) "/Game/StarterContent/Architecture/Wall_400x400.Wall_400x400")
            (Rendering|Material|SetMaterial (Variables|/Script/Engine.StaticMeshActor|GetStaticMeshComponent _returnvalue_7) 0 "/Game/StarterContent/Materials/M_Wood_Pine.M_Wood_Pine")
            (bind _returnvalue_8 (Game|SpawnActorfromClass "/Script/Engine.StaticMeshActor" (Math|Transform|MakeTransform (Math|Vector|MakeVector (* (Math|Conversions|ToFloat(Integer) (Variables|Default|GetPolygon%20Size)) (Math|Conversions|ToFloat(Integer) (+ (- (Class|MyActor|GetHeight _returnvalue) 1) 1))) (* (Math|Conversions|ToFloat(Integer) _index_5) (Math|Conversions|ToFloat(Integer) (Variables|Default|GetPolygon%20Size))) 0.0) "0,90.000000, 0" "0.250000,1.000000,5.000000") "Undefined" 0 0))
            (Components|StaticMesh|SetStaticMesh (Variables|/Script/Engine.StaticMeshActor|GetStaticMeshComponent _returnvalue_8) "/Game/StarterContent/Architecture/Wall_400x400.Wall_400x400")
            (Rendering|Material|SetMaterial (Variables|/Script/Engine.StaticMeshActor|GetStaticMeshComponent _returnvalue_8) 0 "/Game/StarterContent/Materials/M_Wood_Pine.M_Wood_Pine")))))
    (:then_5
      ;[1 1 1] Generation GoL
      (bind _returnvalue_9 (Actor|GetActorOfClass "/Script/Prototype.GoLUser"))
      ;;[1 1 1] There you can set Birth's and Survive's values
      (Class|MyActor|SetBirth _returnvalue (Utilities|Array|MakeArray false false false true false false false false false))
      (Class|MyActor|SetSurvive _returnvalue (Utilities|Array|MakeArray false false true true false false false false false))
      (bind _returnvalue_10 (Class|MyActor|GetBirth _returnvalue))
      (bind _returnvalue_11 (Class|MyActor|GetSurvive _returnvalue))
      (if _tutor
        (Class|GoLUser|GenerateGoLTutorial _returnvalue_9 (+ (- (Class|MyActor|GetWidth _returnvalue) 1) 1) (+ (- (Class|MyActor|GetHeight _returnvalue) 1) 1) _returnvalue_10 _returnvalue_11 _returnvalue)
        (Class|GoLUser|UpdateGoL _returnvalue_9 _returnvalue_10 _returnvalue_11 _returnvalue 1 false _tutor)
        (else
          (Class|GoLUser|GenerateGoL _returnvalue_9 (+ (- (Class|MyActor|GetWidth _returnvalue) 1) 1) (+ (- (Class|MyActor|GetHeight _returnvalue) 1) 1) _returnvalue_10 _returnvalue_11 _returnvalue 1 false)
          ;;[1 1 1] If you think that you need this. Set Last Index value, and the GoL will be updated Last Index times
          (for _index_6 (range 1 5)
            (Class|GoLUser|UpdateGoL _returnvalue_9 _returnvalue_10 _returnvalue_11 _returnvalue 1 false false))
          (Class|GoLUser|ClearCreaturesSpace _returnvalue_9 _returnvalue 1)))
      (Class|GoLUser|UpdateLavaPiecesonField _returnvalue_9 (Variables|Default|GetPolygon%20Size)))
    (:then_6
      ;[1 1 1] Creation of start and finish
      (Utilities|FlowControl|Sequence
        (:then_0
          (bind _returnvalue_12 (Actor|GetActorOfClass "/Game/Blueprints/PlayerPawnmy.PlayerPawnmy_C"))
          (Transformation|SetActorLocation _returnvalue_12 (* (+ (Math|Conversions|ToVector(Float) (Class|MyActor|GetStartPosition _returnvalue)) "0.500000,0.500000,0.000000") (Math|Conversions|ToFloat(Integer) (Variables|Default|GetPolygon%20Size))) false false)
          (bind _output_get_3 (Variables|/Game/Blueprints/Creature.Creature_C|SetPosition _returnvalue_12 (Class|MyActor|GetStartPosition _returnvalue)))
          (Class|MyActor|SetCellIsOccupied _returnvalue (.x _output_get_3) (.y _output_get_3) 2))
        (:then_1
          (bind _returnvalue_13 (Game|SpawnActorfromClass "/Game/Blueprints/Block.Block_C" (Math|Transform|MakeTransform (* (+ (Math|Conversions|ToVector(Float) (Class|MyActor|GetFinishPosition _returnvalue)) "0.500000,0.500000,0.000000") (Math|Conversions|ToFloat(Integer) (Variables|Default|GetPolygon%20Size))) "0, 0, 0" "1,1,1") "Undefined" 0 (Class|MyActor|GetFinishPosition _returnvalue) 0))
          (Components|StaticMesh|SetStaticMesh (Variables|/Game/Blueprints/Block.Block_C|GetCube _returnvalue_13) "/Engine/Functions/Engine_MaterialFunctions02/ExampleContent/PivotPainter2/SimplePivotPainterExample.SimplePivotPainterExample")
          (Rendering|Material|SetMaterial (Variables|/Game/Blueprints/Block.Block_C|GetCube _returnvalue_13) 0 "/Game/StarterContent/Materials/M_Wood_Oak.M_Wood_Oak"))))
    (:then_7
      (if (Variables|Default|GetTutor) ; On/Off enemies
        (bind _returnvalue_14 (Game|SpawnActorfromClass "/Game/Blueprints/NPCNew.NPCNew_C" (Math|Transform|MakeTransform (* (+ (Math|Conversions|ToVector(Float) (Class|MyActor|GetFinishPosition _returnvalue)) "0.500000,-2.500000,0.000000") (Math|Conversions|ToFloat(Integer) (Variables|Default|GetPolygon%20Size))) "0, 0, 0" "1,1,1") "Undefined" 0 0))
        (bind _output_get_4 (Variables|/Game/Blueprints/Creature.Creature_C|SetPosition _returnvalue_14 (Class|KismetMathLibrary|FTruncVector (+ (Math|Conversions|ToVector(Float) (Class|MyActor|GetFinishPosition _returnvalue)) "0.500000,-2.500000,0.000000"))))
        (Actor|GetActorOfClass "/Game/Blueprints/Turn-Based.Turn-Based_C")
        (Class|MyActor|SetCellIsOccupied _returnvalue (.x _output_get_4) (.y _output_get_4) 2)
        (else
          ;[1 1 1] Creation of NPCs
          (for _index_7 (range 0 (- (Variables|/Game/Blueprints/Global.Global_C|GetGNumOfEnemies _asglobal) 1))
            (bind _returnvalue_15 (Game|SpawnActorfromClass "/Game/Blueprints/NPCNew.NPCNew_C" (Math|Transform|MakeTransform (* (+ (Math|Conversions|ToVector(Float) (Class|MyActor|GetEnemyPosition _returnvalue _index_7)) "0.500000,0.500000,0.000000") (Math|Conversions|ToFloat(Integer) (Variables|Default|GetPolygon%20Size))) "0, 0, 0" "1,1,1") "Undefined" 0 0))
            (bind _output_get_5 (Variables|/Game/Blueprints/Creature.Creature_C|SetPosition _returnvalue_15 (Class|MyActor|GetEnemyPosition _returnvalue _index_7)))
            (bind _returnvalue_16 (Actor|GetActorOfClass "/Game/Blueprints/Turn-Based.Turn-Based_C"))
            (Class|MyActor|SetCellIsOccupied _returnvalue (.x _output_get_5) (.y _output_get_5) 2)))))))

(event EventTick
  (params (DeltaSeconds :type Float%20%28single-precision%29)))

(event Collision|EventActorBeginOverlap
  (params (OtherActor :type Actor%20Object%20Reference)))

(fn ConstructionScript)

(fn FLOORGENERATOR
  (params (Polygon%20size :type Integer) (Height :type Integer) (WIdth :type Integer) (UV%20Scale :type Float%20%28single-precision%29))
  (bind _returnvalue (- WIdth 1))
  (bind _returnvalue_2 (- Height 1))
  (Utilities|Array|Clear (Variables|Default|GetVERTICES))
  (Utilities|Array|Clear (Variables|Default|GetTRIANGLES))
  (for _index (range 0 _returnvalue_2)
    (for _index_2 (range 0 _returnvalue)
      (Utilities|FlowControl|Sequence
        (:then_0
          ;[1 1 1] Vertices
          (Utilities|Array|Add (Variables|Default|GetVERTICES) (Math|Vector|MakeVector (Math|Conversions|ToFloat(Integer) (* _index Polygon%20size)) (Math|Conversions|ToFloat(Integer) (* _index_2 Polygon%20size)) 0.0)))
        (:then_1
          ;[1 1 1] Triangles
          (if (and (!= _index _returnvalue_2) (!= _index_2 _returnvalue))
            (Class|KismetProceduralMeshLibrary|ConvertQuadtoTriangles (Variables|Default|GetTRIANGLES) (+ _index_2 (* _index WIdth)) (+ (+ _index_2 (* _index WIdth)) 1) (+ (+ _index_2 (* (+ _index 1) WIdth)) 1) (+ _index_2 (* (+ _index 1) WIdth)))))
        (:then_2
          ;[1 1 1] UV
          (Utilities|Array|Add (Variables|Default|GetUV) (Math|Vector2D|MakeVector2D (* (/ 1.0 (Math|Conversions|ToFloat(Integer) _returnvalue_2)) (Math|Conversions|ToFloat(Integer) _index) UV%20Scale) (* UV%20Scale (Math|Conversions|ToFloat(Integer) _index_2) (/ 1.0 (Math|Conversions|ToFloat(Integer) _returnvalue))))))))))