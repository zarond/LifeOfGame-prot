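; Turn-based grid NPC that detects and fights the player and other NPCs, and wanders when it has no targets.
; EnemyTurn spends one substep per call, then reloads move, attack and defence from its behaviour object.
; Targets come from radius scans and attackers, are attacked within Manhattan range, or chased greedily without pathfinding.
; Movement avoids GoLUser cells that are or will be alive, and death frees the cell and unregisters the NPC.
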(event Collision|EventActorBeginOverlap
  (params (OtherActor :type Actor%20Object%20Reference)))

(event EventTick
  (params (DeltaSeconds :type Float%20%28single-precision%29)))

(event EventBeginPlay
  (bind _returnvalue (AddComponent|AddBehaviour))
  (Variables|Default|SetBehaviourClass _returnvalue)
  (switch int (Math|Random|RandomInteger 3)
    (:0
      (Variables|Default|SetTo%20Move (Utilities|Struct|MakeIntVector 1 0)))
    (:1
      (Variables|Default|SetTo%20Move (Utilities|Struct|MakeIntVector 0 1)))
    (:2
      (Variables|Default|SetTo%20Move (Utilities|Struct|MakeIntVector -1 0)))
    (:3
      (Variables|Default|SetTo%20Move (Utilities|Struct|MakeIntVector 0 -1)))))

(fn ConstructionScript)

(fn EnemyTurn
  (bind _arrayoftargets (Variables|Default|GetArrayOfTargets))
  (bind _behaviourclass (Variables|Default|GetBehaviourClass))
  ;[1 1 1] Жив ли вообще
  (if (>= (Variables|Default|GetHP) 0)
    (if (> (Variables|Default|GetNumber%20Of%20Remaining%20Substeps) 0)
      ;[1 1 1] Действия за сабстеп
      (Development|PrintString (Utilities|String|Append "SUBSTEPS:" (Utilities|String|ToString(Integer) (Variables|Default|GetNumber%20Of%20Remaining%20Substeps))) true true "(R=1.000000,G=0.983937,B=0.000000,A=1.000000)")
      (Math|Integer|DecrementInt (Variables|Default|GetNumber%20Of%20Remaining%20Substeps)
        (:%20%20
          (CallFunction|CheckSurroundings)
          (bind _output_get (Variables|Default|SetIs%20in%20combat (> (Utilities|Array|Length (Variables|Default|GetArrayOfTargets)) 0)))
          (if _output_get
            ;;[0.5869 1 0.6123] Сколько целей вообще осталось в живых(=надо ли оставаться в бою)
            (for _array_element _arrayoftargets
              (if (not (Utilities|IsValid _array_element))
                (Utilities|Array|RemoveItem _arrayoftargets _array_element))))
          (bind _output_get_2 (Variables|Default|SetIs%20in%20combat (> (Utilities|Array|Length (Variables|Default|GetArrayOfTargets)) 0)))
          (if _output_get_2
            (Development|PrintString "IN BATTLE!" true true "(R=0.000000,G=0.982796,B=1.000000,A=1.000000)")
            (bind _couldattack (CallFunction|TryAttack))
            (if _couldattack
              _
              (elif (> (Variables|Default|GetmoveAmount) 0)
                (CallFunction|TryFollow)))
            (else
              (Development|PrintString "Peace" true true "(R=0.000000,G=1.000000,B=0.812759,A=1.000000)")
              (if (> (Variables|Default|GetmoveAmount) 0)
                (CallFunction|Wander))))
          (if (> (Variables|Default|GetNumber%20Of%20Remaining%20Substeps) 0)
            (return (> (Variables|Default|GetNumber%20Of%20Remaining%20Substeps) 0))
            (else
              _)))))
    ;[1 1 1] Получение параметров из боевой матрицы
    (Development|PrintString "Setting parameters" true true "(R=0.000000,G=0.951603,B=1.000000,A=1.000000)")
    (Utilities|FlowControl|Sequence
      (:then_0
        (bind _returnvalue (Class|Behaviour|GetMove _behaviourclass))
        (bind _output_get_3 (Variables|Default|SetmoveAmount _returnvalue))
        (Variables|Default|SetNumber%20Of%20Remaining%20Substeps _output_get_3))
      (:then_1
        (bind _returnvalue_2 (Class|Behaviour|GetAttack _behaviourclass))
        (Variables|Default|SetbaseAttack _returnvalue_2))
      (:then_2
        (bind _returnvalue_3 (Class|Behaviour|GetDefence _behaviourclass))
        (Variables|Default|SetbaseDefense _returnvalue_3))
      (:then_3
        (Development|PrintString "EnemyAction")
        (bind _returnvalue_4 (Class|Behaviour|GetSubsteps _behaviourclass))
        (Development|PrintString (Utilities|String|Append (LocalVariables|GetMoveWord) (Utilities|String|ToString(Integer) _returnvalue)))
        (Development|PrintString (Utilities|String|Append (LocalVariables|GetAttackWord) (Utilities|String|ToString(Integer) _returnvalue_2)))
        (Development|PrintString (Utilities|String|Append (LocalVariables|GetDefenceWord) (Utilities|String|ToString(Integer) _returnvalue_3)))
        (Class|Behaviour|NextStep _behaviourclass)
        (Class|Behaviour|SetSubsteps _behaviourclass 3)
        (bind _returnvalue_5 (Class|Behaviour|GetSubsteps _behaviourclass))
        (return false)))
    (else
      (CallFunction|Die))))

(fn ReceiveDamage
  (params (Damage :type Integer) (Attacker :type Creature%20Object%20Reference))
  (bind _diddie (CallFunction|ReceiveDamageBase Damage))
  (if _diddie
    (CallFunction|Die)
    (return true)
    (else
      (Variables|Default|SetIs%20in%20combat true)
      (Utilities|Array|AddUnique (Variables|Default|GetArrayOfTargets) Attacker)
      (return false))))

(fn Die
  (bind _self self)
  (bind _position (Variables|Default|GetPosition))
  (bind (_x _y) (Utilities|Struct|BreakIntVector _position))
  (bind _returnvalue (Actor|GetActorOfClass "/Game/Blueprints/Turn-Based.Turn-Based_C"))
  (bind _returnvalue_2 (Actor|GetActorOfClass "/Script/Prototype.MyActor"))
  (Development|PrintString (Utilities|String|Append (Utilities|String|ToString(Integer) (Utilities|Array|FindItem (Variables|/Game/Blueprints/Turn-Based.Turn-Based_C|GetArrayOfNPCs _returnvalue) _self)) "died") true true "(R=1.000000,G=0.043376,B=0.000000,A=1.000000)")
  (Class|MyActor|SetCellIsOccupied _returnvalue_2 _x _y)
  (Utilities|Array|RemoveItem (Variables|/Game/Blueprints/Turn-Based.Turn-Based_C|GetArrayOfNPCs _returnvalue) _self)
  (Actor|DestroyActor))

(fn Attack
  (params (Target :type Creature%20Object%20Reference))
  (bind _returnvalue (Utilities|GetClass Target))
  (bind _baseattack (Variables|Default|GetbaseAttack))
  (Development|PrintString "PEW" true true "(R=0.000000,G=0.848144,B=1.000000,A=1.000000)")
  (if (== _returnvalue "/Game/Blueprints/PlayerPawn.PlayerPawn_C")
    (bind _asplayer_pawn (Utilities|Casting|CastToPlayerPawn Target))
    (bind _diddie (Default|ReceiveDamage _asplayer_pawn _baseattack))
    (if (or _diddie (stale _diddie_2)) :!label _label
      (Development|PrintString "ENEMY TERMINATED" true true "(R=0.177083,G=0.124511,B=0.127853,A=1.000000)")
      (Utilities|Array|RemoveItem (Variables|Default|GetArrayOfTargets) Target))
    (elif (== _returnvalue "NPC_C")
      (bind _asnpc (Utilities|Casting|CastToNPC Target))
      (bind _diddie_2 (CallFunction|ReceiveDamage _asnpc _baseattack self))
      (goto _label))))

(fn Wander
  (bind _position (Variables|Default|GetPosition))
  (bind (_x _y) (Utilities|Struct|BreakIntVector _position))
  (bind _returnvalue (Actor|GetActorOfClass "/Script/Prototype.GoLUser"))
  (Utilities|FlowControl|ForLoopwithBreak 0 8 :!label _label
    (:LoopBody
      (if (or (Class|GoLUser|IsAlive _returnvalue (+ _x (.X (Utilities|Struct|BreakIntVector (Variables|Default|GetTo%20Move)))) (+ _y (.Y (Utilities|Struct|BreakIntVector (Variables|Default|GetTo%20Move))))) (Class|GoLUser|WillbeAlive _returnvalue (+ _x (.X (Utilities|Struct|BreakIntVector (Variables|Default|GetTo%20Move)))) (+ _y (.Y (Utilities|Struct|BreakIntVector (Variables|Default|GetTo%20Move))))))
        _
        (else
          (bind _success (CallFunction|TryMove (Variables|Default|GetTo%20Move)))
          (if _success
            (goto _label Break)
            (else
              _))))
      (bind _new (CallFunction|ChangeDirection (Variables|Default|GetTo%20Move)))
      (Variables|Default|SetTo%20Move _new))
    (:Completed
      (Development|PrintString "Walking~~~~~" true true "(R=0.000000,G=0.947419,B=1.000000,A=1.000000)"))))

(fn ChangeDirection
  (params (Prev :type Int%20Vector%20Structure))
  (bind (_x _y) (Utilities|Struct|BreakIntVector Prev))
  (bind _returnvalue (Math|Random|RandomInteger 3))
  (if (!= _x 0)
    (switch int _returnvalue
      (:Default
        (return (Utilities|Struct|MakeIntVector (* _x -1) 0 0)))
      (:0
        (return (Utilities|Struct|MakeIntVector 0 -1 0)))
      (:1
        (return (Utilities|Struct|MakeIntVector 0 1 0))))
    (else
      (switch int _returnvalue
        (:Default
          (return (Utilities|Struct|MakeIntVector 0 (* _y -1) 0)))
        (:0
          (return (Utilities|Struct|MakeIntVector -1 0 0)))
        (:1
          (return (Utilities|Struct|MakeIntVector -1 0 0)))))))

(fn TryAttack
  (bind _arrayoftargets (Variables|Default|GetArrayOfTargets))
  (bind _position (Variables|Default|GetPosition))
  (bind (_x _y) (Utilities|Struct|BreakIntVector _position))
  (bind _array_element (Utilities|Array|ForEachLoopwithBreak _arrayoftargets)
    (:LoopBody
      (if (Utilities|IsValid _array_element)
        (if (<= (+ (Math|Integer|Absolute(Integer) (- (.X (Utilities|Struct|BreakIntVector (Variables|/Game/Blueprints/Creature.Creature_C|GetPosition _array_element))) _x)) (Math|Integer|Absolute(Integer) (- (.Y (Utilities|Struct|BreakIntVector (Variables|/Game/Blueprints/Creature.Creature_C|GetPosition _array_element))) _y))) (Variables|Default|GetattackRadius))
          (CallFunction|Attack _array_element)
          (return true))
        (else
          (Utilities|Array|RemoveItem _arrayoftargets _array_element))))
    (:Completed
      (return false))))

(fn Follow
  (params (Target :type Creature%20Object%20Reference))
  (bind _position (Variables|/Game/Blueprints/Creature.Creature_C|GetPosition Target))
  (bind _position_2 (Variables|Default|GetPosition))
  (bind _position_3 (Variables|Default|GetPosition))
  (bind (_x _y) (Utilities|Struct|BreakIntVector _position_2))
  (bind (_x_2 _y_2) (Utilities|Struct|BreakIntVector _position))
  (bind (_x_3 _y_3) (Utilities|Struct|BreakIntVector _position_3))
  (bind _returnvalue (Actor|GetActorOfClass "/Script/Prototype.GoLUser"))
  (if (> _x_2 _x_3)
    (bind _output_get (Variables|Default|SetTo%20Move (Utilities|Struct|MakeIntVector 1 0)))
    (if (or (Class|GoLUser|IsAlive _returnvalue (+ _x (.X (Utilities|Struct|BreakIntVector (Variables|Default|GetTo%20Move)))) (+ _y (.Y (Utilities|Struct|BreakIntVector (Variables|Default|GetTo%20Move))))) (Class|GoLUser|WillbeAlive _returnvalue (+ _x (.X (Utilities|Struct|BreakIntVector (Variables|Default|GetTo%20Move)))) (+ _y (.Y (Utilities|Struct|BreakIntVector (Variables|Default|GetTo%20Move))))))
      (if (< _x_2 _x_3) :!label _label
        (bind _output_get_2 (Variables|Default|SetTo%20Move (Utilities|Struct|MakeIntVector -1 0)))
        (if (or (Class|GoLUser|IsAlive _returnvalue (+ _x (.X (Utilities|Struct|BreakIntVector (Variables|Default|GetTo%20Move)))) (+ _y (.Y (Utilities|Struct|BreakIntVector (Variables|Default|GetTo%20Move))))) (Class|GoLUser|WillbeAlive _returnvalue (+ _x (.X (Utilities|Struct|BreakIntVector (Variables|Default|GetTo%20Move)))) (+ _y (.Y (Utilities|Struct|BreakIntVector (Variables|Default|GetTo%20Move))))))
          (if (> _y_2 _y_3) :!label _label_2
            (bind _output_get_3 (Variables|Default|SetTo%20Move (Utilities|Struct|MakeIntVector 0 1)))
            (if (or (Class|GoLUser|IsAlive _returnvalue (+ _x (.X (Utilities|Struct|BreakIntVector (Variables|Default|GetTo%20Move)))) (+ _y (.Y (Utilities|Struct|BreakIntVector (Variables|Default|GetTo%20Move))))) (Class|GoLUser|WillbeAlive _returnvalue (+ _x (.X (Utilities|Struct|BreakIntVector (Variables|Default|GetTo%20Move)))) (+ _y (.Y (Utilities|Struct|BreakIntVector (Variables|Default|GetTo%20Move))))))
              (if (< _y_2 _y_3) :!label _label_3
                (bind _output_get_4 (Variables|Default|SetTo%20Move (Utilities|Struct|MakeIntVector 0 -1)))
                (if (or (Class|GoLUser|IsAlive _returnvalue (+ _x (.X (Utilities|Struct|BreakIntVector (Variables|Default|GetTo%20Move)))) (+ _y (.Y (Utilities|Struct|BreakIntVector (Variables|Default|GetTo%20Move))))) (Class|GoLUser|WillbeAlive _returnvalue (+ _x (.X (Utilities|Struct|BreakIntVector (Variables|Default|GetTo%20Move)))) (+ _y (.Y (Utilities|Struct|BreakIntVector (Variables|Default|GetTo%20Move))))))
                  (return false)
                  (else
                    (bind _success (CallFunction|TryMove _output_get_4))
                    (if _success
                      (return true)
                      (else
                        (return false))))))
              (else
                (bind _success_2 (CallFunction|TryMove _output_get_3))
                (if _success_2
                  (return true)
                  (else
                    (goto _label_3)))))
            (else
              (goto _label_3)))
          (else
            (bind _success_3 (CallFunction|TryMove _output_get_2))
            (if _success_3
              (return true)
              (else
                (goto _label_2)))))
        (else
          (goto _label_2)))
      (else
        (bind _success_4 (CallFunction|TryMove _output_get))
        (if _success_4
          (return true)
          (else
            (goto _label)))))
    (else
      (goto _label))))

(fn CheckSurroundings
  (bind _position (Variables|Default|GetPosition))
  (bind _position_2 (Variables|Default|GetPosition))
  (bind (_x _y) (Utilities|Struct|BreakIntVector _position))
  (bind (_x_2 _y_2) (Utilities|Struct|BreakIntVector _position_2))
  (Development|PrintString "Looking around------------" true true "(R=0.000000,G=0.505208,B=0.489775,A=1.000000)")
  (bind _returnvalue (Actor|GetActorOfClass "/Game/Blueprints/PlayerPawn.PlayerPawn_C"))
  (if (<= (+ (Math|Integer|Absolute(Integer) (- (.X (Utilities|Struct|BreakIntVector (Variables|/Game/Blueprints/Creature.Creature_C|GetPosition _returnvalue))) _x)) (Math|Integer|Absolute(Integer) (- (.Y (Utilities|Struct|BreakIntVector (Variables|/Game/Blueprints/Creature.Creature_C|GetPosition _returnvalue))) _y))) (Variables|Default|GetdetectRadius))
    (Utilities|Array|AddUnique (Variables|Default|GetArrayOfTargets) _returnvalue)
    (return)
    (else
      (bind _returnvalue_2 (Actor|GetActorOfClass "/Game/Blueprints/Turn-Based.Turn-Based_C"))
      (bind _array_element (Utilities|Array|ForEachLoopwithBreak (Variables|/Game/Blueprints/Turn-Based.Turn-Based_C|GetArrayOfNPCs _returnvalue_2))
        (:LoopBody
          (if (and (<= (+ (Math|Integer|Absolute(Integer) (- (.X (Utilities|Struct|BreakIntVector (Variables|/Game/Blueprints/Creature.Creature_C|GetPosition _array_element))) _x_2)) (Math|Integer|Absolute(Integer) (- (.Y (Utilities|Struct|BreakIntVector (Variables|/Game/Blueprints/Creature.Creature_C|GetPosition _array_element))) _y_2))) (Variables|Default|GetdetectRadius)) (or (> (Math|Integer|Absolute(Integer) (- (.X (Utilities|Struct|BreakIntVector (Variables|/Game/Blueprints/Creature.Creature_C|GetPosition _array_element))) _x_2)) 0) (> (Math|Integer|Absolute(Integer) (- (.Y (Utilities|Struct|BreakIntVector (Variables|/Game/Blueprints/Creature.Creature_C|GetPosition _array_element))) _y_2)) 0)))
            (Utilities|Array|AddUnique (Variables|Default|GetArrayOfTargets) _array_element)))
        (:Completed
          (return))))))

(fn TryFollow
  ;[1 1 1] Попытка следовать
  (bind _array_element (Utilities|Array|ForEachLoopwithBreak (Variables|Default|GetArrayOfTargets))
    (:LoopBody
      (if (Utilities|IsValid _array_element)
        (CallFunction|Follow _array_element)
        (Development|PrintString "chaaaaaaaaaaarge" true true "(R=0.000000,G=0.626957,B=0.651042,A=1.000000)" :!label _label)
        (Math|Integer|DecrementInt (Variables|Default|GetmoveAmount)
          (:%20%20
            (return)))))
    (:Completed
      (Development|PrintString "No valid targets")
      (goto _label))))