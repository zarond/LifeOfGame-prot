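; Player pawn for a turn-based grid game that moves cell by cell and collects pickups.
; Directional inputs spend substeps through TryMove, where CheckIfBlocked returns true for in-bounds free cells in the game mode's flattened Cells array.
; Successful moves call TryPickUp, which compares only the first pickup's position before returning, then notify the Turn-Based game mode via NextSubstep.
; Enter refills substeps from Speed and calls NextStep.
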(event EventBeginPlay
  ;[1 1 1] Initial assignments
  (bind _asturn__based (Utilities|Casting|CastToTurn-Based (Game|GetGameMode)))
  (Variables|Default|SetGameMode _asturn__based))

(event Collision|EventActorBeginOverlap
  (params (OtherActor :type Actor%20Object%20Reference)))

(event EventTick
  (params (DeltaSeconds :type Float%20%28single-precision%29)))

(event Input|ActionEvents|InputActionEnter
  (params (Key :type Key%20Structure :default "None"))
  ;[1 1 1] Обработка input событий
  (:Pressed
    (Variables|Default|SetNumber%20Of%20Remaining%20Substeps (Variables|Default|GetSpeed))
    (Default|NextStep (Variables|Default|GetGameMode) self)))

(event Input|ActionEvents|InputActionMoveUp
  (params (Key :type Key%20Structure :default "None"))
  (bind _position (Variables|Default|GetPosition))
  (bind (_x _y) (Utilities|Struct|BreakIntVector _position))
  ;[1 1 1] Обработка input событий
  (:Pressed
    (if (> (Variables|Default|GetNumber%20Of%20Remaining%20Substeps) 0)
      (Variables|Default|SetToMove (Utilities|Struct|MakeIntVector 1 0))
      (bind _success (CallFunction|TryMove (Variables|Default|GetToMove)))
      (if _success
        (CallFunction|TryPickUp)
        (Development|PrintString (Utilities|String|Append (Utilities|String|Append (Utilities|String|ToString(Integer) _x) " ") (Utilities|String|ToString(Integer) _y)) true true "(R=1.000000,G=0.114357,B=0.113036,A=1.000000)")
        (Default|NextSubstep (Variables|Default|GetGameMode) self) ; После передвижения и пикапа вызывается следующий подшаг
        (Math|Integer|DecrementInt (Variables|Default|GetNumber%20Of%20Remaining%20Substeps))))))

(event Input|ActionEvents|InputActionMoveDown
  (params (Key :type Key%20Structure :default "None"))
  (bind _position (Variables|Default|GetPosition))
  (bind (_x _y) (Utilities|Struct|BreakIntVector _position))
  ;[1 1 1] Обработка input событий
  (:Pressed
    (if (> (Variables|Default|GetNumber%20Of%20Remaining%20Substeps) 0)
      (Variables|Default|SetToMove (Utilities|Struct|MakeIntVector -1 0))
      (bind _success (CallFunction|TryMove (Variables|Default|GetToMove)))
      (if _success
        (CallFunction|TryPickUp)
        (Development|PrintString (Utilities|String|Append (Utilities|String|Append (Utilities|String|ToString(Integer) _x) " ") (Utilities|String|ToString(Integer) _y)) true true "(R=1.000000,G=0.114357,B=0.113036,A=1.000000)")
        (Default|NextSubstep (Variables|Default|GetGameMode) self) ; После передвижения и пикапа вызывается следующий подшаг
        (Math|Integer|DecrementInt (Variables|Default|GetNumber%20Of%20Remaining%20Substeps))))))

(event Input|ActionEvents|InputActionMoveLeft
  (params (Key :type Key%20Structure :default "None"))
  (bind _position (Variables|Default|GetPosition))
  (bind (_x _y) (Utilities|Struct|BreakIntVector _position))
  ;[1 1 1] Обработка input событий
  (:Pressed
    (if (> (Variables|Default|GetNumber%20Of%20Remaining%20Substeps) 0)
      (Variables|Default|SetToMove (Utilities|Struct|MakeIntVector 0 -1))
      (bind _success (CallFunction|TryMove (Variables|Default|GetToMove)))
      (if _success
        (CallFunction|TryPickUp)
        (Development|PrintString (Utilities|String|Append (Utilities|String|Append (Utilities|String|ToString(Integer) _x) " ") (Utilities|String|ToString(Integer) _y)) true true "(R=1.000000,G=0.114357,B=0.113036,A=1.000000)")
        (Default|NextSubstep (Variables|Default|GetGameMode) self) ; После передвижения и пикапа вызывается следующий подшаг
        (Math|Integer|DecrementInt (Variables|Default|GetNumber%20Of%20Remaining%20Substeps))))))

(event Input|ActionEvents|InputActionMoveRight
  (params (Key :type Key%20Structure :default "None"))
  (bind _position (Variables|Default|GetPosition))
  (bind (_x _y) (Utilities|Struct|BreakIntVector _position))
  ;[1 1 1] Обработка input событий
  (:Pressed
    (if (> (Variables|Default|GetNumber%20Of%20Remaining%20Substeps) 0)
      (Variables|Default|SetToMove (Utilities|Struct|MakeIntVector 0 1))
      (bind _success (CallFunction|TryMove (Variables|Default|GetToMove)))
      (if _success
        (CallFunction|TryPickUp)
        (Development|PrintString (Utilities|String|Append (Utilities|String|Append (Utilities|String|ToString(Integer) _x) " ") (Utilities|String|ToString(Integer) _y)) true true "(R=1.000000,G=0.114357,B=0.113036,A=1.000000)")
        (Default|NextSubstep (Variables|Default|GetGameMode) self) ; После передвижения и пикапа вызывается следующий подшаг
        (Math|Integer|DecrementInt (Variables|Default|GetNumber%20Of%20Remaining%20Substeps))))))

(fn ConstructionScript)

(fn TryMove
  (params (MoveV :type Int%20Vector%20Structure))
  (bind (_x _y) (Utilities|Struct|BreakIntVector MoveV))
  (bind (_x_2 _y_2) (Utilities|Struct|BreakIntVector MoveV))
  (bind _gamemode (Variables|Default|GetGameMode))
  (bind _polygon_size (Variables|/Game/Blueprints/Turn-Based.Turn-Based_C|GetPolygon%20Size _gamemode))
  (bind _returnvalue (Math|Conversions|ToFloat(Integer) _polygon_size))
  (bind _free (CallFunction|CheckifBlocked (Utilities|Struct|MakeIntVector (+ _x (.X (Utilities|Struct|BreakIntVector (Variables|Default|GetPosition)))) (+ _y (.Y (Utilities|Struct|BreakIntVector (Variables|Default|GetPosition)))))))
  (if _free
    (Transformation|AddActorLocalOffset (Math|Vector|MakeVector (* _x_2 _returnvalue) (* _y_2 _returnvalue) 0.0) false false)
    (Variables|Default|SetPosition (Utilities|Struct|MakeIntVector (+ _x (.X (Utilities|Struct|BreakIntVector (Variables|Default|GetPosition)))) (+ _y (.Y (Utilities|Struct|BreakIntVector (Variables|Default|GetPosition))))))
    (return true)
    (else
      (return false))))

(fn CheckifBlocked
  (params (Position :type Int%20Vector%20Structure))
  (bind _gamemode (Variables|Default|GetGameMode))
  (bind _output_get (LocalVariables|SetWidth (Variables|/Game/Blueprints/Turn-Based.Turn-Based_C|GetWidth _gamemode)))
  (bind _output_get_2 (LocalVariables|SetHeight (Variables|/Game/Blueprints/Turn-Based.Turn-Based_C|GetHeight _gamemode)))
  (if (Math|Boolean|ORBoolean (< (.x Position) 0) (>= (.x Position) _output_get) (< (.y Position) 0) (>= (.y Position) _output_get_2))
    _
    (elif (== (.isbusy (Utilities|Array|Get(acopy) (Variables|/Game/Blueprints/Turn-Based.Turn-Based_C|GetCells _gamemode) (+ (.y Position) (* (.x Position) _output_get_2)))) 0)
      (return true)
      (else
        _)))
  (return false))

(fn TryPickUp
  (bind _position (Variables|Default|GetPosition))
  (bind (_x _y) (Utilities|Struct|BreakIntVector _position))
  (bind _array_element (Utilities|Array|ForEachLoopwithBreak (Variables|/Game/Blueprints/Turn-Based.Turn-Based_C|GetArrayOfPickUps (Variables|Default|GetGameMode)))
    (:LoopBody
      (if (and (== (.X (Utilities|Struct|BreakIntVector (Variables|/Game/Blueprints/PickUp.PickUp_C|GetPosition _array_element))) _x) (== (.Y (Utilities|Struct|BreakIntVector (Variables|/Game/Blueprints/PickUp.PickUp_C|GetPosition _array_element))) _y))
        (Default|PickUp _array_element)
        (return true)
        (else
          (return false))))))