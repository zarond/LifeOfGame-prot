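; Grid-based creature actor that moves, attacks, picks up items and dies, spending substeps on moves and attacks.
; TryMove updates cell occupancy on MyActor, then Tick glides and turns the actor toward the cell centre, scaled by Procedual's PolygonSize.
; TryAttack hits the creature at an offset cell; ReceiveDamage subtracts defense, spawns effects and floating text, and Die frees the cell.
; A health widget and hover-toggled InfoVisualiser show creature info.
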(event EventBeginPlay
  (CallFunction|SetHealthWidget))

(event MouseInput|EventActorBeginCursorOver
  (Default|On (Variables|Default|GetInfoVisualiser)))

(event MouseInput|EventActorEndCursorOver
  (Default|Off (Variables|Default|GetInfoVisualiser)))

(event EventDestroyed
  (Default|Off (Variables|Default|GetInfoVisualiser)))

(event Custom|FinishMove
  (Variables|Default|SetMoving false)
  (Development|PrintString "Goodbye"))

(event Custom|StartMove
  (Variables|Default|SetMoving true)
  (Development|PrintString "Hello"))

(event EventBeginPlay
  ;[1 1 1] Initial assignments
)

(event Collision|EventActorBeginOverlap
  (params (OtherActor :type Actor%20Object%20Reference)))

(event EventTick
  (params (DeltaSeconds :type Float%20%28single-precision%29))
  (bind _returnvalue (Actor|GetActorOfClass "/Game/Blueprints/PROCEDUAL.Procedual_C"))
  (Variables|Default|SetVel (* (Math|Vector|Normalize (- (Math|Vector|MakeVector (.X (Math|Vector|BreakVector (* (+ (Math|Conversions|ToVector(Float) (Variables|BattleCharacteristics|GetPosition)) "0.500000,0.500000,1.000000") (Math|Conversions|ToFloat(Integer) (Variables|/Game/Blueprints/PROCEDUAL.Procedual_C|GetPolygon%20Size _returnvalue))))) (.Y (Math|Vector|BreakVector (* (+ (Math|Conversions|ToVector(Float) (Variables|BattleCharacteristics|GetPosition)) "0.500000,0.500000,1.000000") (Math|Conversions|ToFloat(Integer) (Variables|/Game/Blueprints/PROCEDUAL.Procedual_C|GetPolygon%20Size _returnvalue))))) (.Z (Math|Vector|BreakVector (Transformation|GetActorLocation)))) (Transformation|GetActorLocation))) (Variables|Default|Getvelocity)))
  (if (Variables|Default|GetMoving)
    (if (<= (* (Variables|Default|Getvelocity) DeltaSeconds) (Math|Vector|VectorLength (- (Math|Vector|MakeVector (.X (Math|Vector|BreakVector (* (+ (Math|Conversions|ToVector(Float) (Variables|BattleCharacteristics|GetPosition)) "0.500000,0.500000,1.000000") (Math|Conversions|ToFloat(Integer) (Variables|/Game/Blueprints/PROCEDUAL.Procedual_C|GetPolygon%20Size _returnvalue))))) (.Y (Math|Vector|BreakVector (* (+ (Math|Conversions|ToVector(Float) (Variables|BattleCharacteristics|GetPosition)) "0.500000,0.500000,1.000000") (Math|Conversions|ToFloat(Integer) (Variables|/Game/Blueprints/PROCEDUAL.Procedual_C|GetPolygon%20Size _returnvalue))))) (.Z (Math|Vector|BreakVector (Transformation|GetActorLocation)))) (Transformation|GetActorLocation))))
      (Transformation|AddWorldOffset (Variables|Default|GetDefaultSceneRoot) (* (* (Math|Vector|Normalize (- (Math|Vector|MakeVector (.X (Math|Vector|BreakVector (* (+ (Math|Conversions|ToVector(Float) (Variables|BattleCharacteristics|GetPosition)) "0.500000,0.500000,1.000000") (Math|Conversions|ToFloat(Integer) (Variables|/Game/Blueprints/PROCEDUAL.Procedual_C|GetPolygon%20Size _returnvalue))))) (.Y (Math|Vector|BreakVector (* (+ (Math|Conversions|ToVector(Float) (Variables|BattleCharacteristics|GetPosition)) "0.500000,0.500000,1.000000") (Math|Conversions|ToFloat(Integer) (Variables|/Game/Blueprints/PROCEDUAL.Procedual_C|GetPolygon%20Size _returnvalue))))) (.Z (Math|Vector|BreakVector (Transformation|GetActorLocation)))) (Transformation|GetActorLocation))) (Variables|Default|Getvelocity)) DeltaSeconds) false false)
      (Transformation|SetActorRotation (Math|Rotator|MakeRotfromXZ (Math|Vector|Normalize (- (Math|Vector|MakeVector (.X (Math|Vector|BreakVector (* (+ (Math|Conversions|ToVector(Float) (Variables|BattleCharacteristics|GetPosition)) "0.500000,0.500000,1.000000") (Math|Conversions|ToFloat(Integer) (Variables|/Game/Blueprints/PROCEDUAL.Procedual_C|GetPolygon%20Size _returnvalue))))) (.Y (Math|Vector|BreakVector (* (+ (Math|Conversions|ToVector(Float) (Variables|BattleCharacteristics|GetPosition)) "0.500000,0.500000,1.000000") (Math|Conversions|ToFloat(Integer) (Variables|/Game/Blueprints/PROCEDUAL.Procedual_C|GetPolygon%20Size _returnvalue))))) (.Z (Math|Vector|BreakVector (Transformation|GetActorLocation)))) (Transformation|GetActorLocation))) (Math|Vector|VectorUp)))
      (else
        (Transformation|SetActorLocation (Math|Vector|MakeVector (.X (Math|Vector|BreakVector (* (+ (Math|Conversions|ToVector(Float) (Variables|BattleCharacteristics|GetPosition)) "0.500000,0.500000,1.000000") (Math|Conversions|ToFloat(Integer) (Variables|/Game/Blueprints/PROCEDUAL.Procedual_C|GetPolygon%20Size _returnvalue))))) (.Y (Math|Vector|BreakVector (* (+ (Math|Conversions|ToVector(Float) (Variables|BattleCharacteristics|GetPosition)) "0.500000,0.500000,1.000000") (Math|Conversions|ToFloat(Integer) (Variables|/Game/Blueprints/PROCEDUAL.Procedual_C|GetPolygon%20Size _returnvalue))))) (.Z (Math|Vector|BreakVector (Transformation|GetActorLocation)))) false false)
        (CallFunction|FinishMove)))))

(fn ConstructionScript)

(fn TryMove
  (params (To%20Move :type Int%20Vector%20Structure))
  (bind (_x _y) (Utilities|Struct|BreakIntVector To%20Move))
  (bind _returnvalue (Actor|GetActorOfClass "/Script/Prototype.MyActor"))
  (if (Class|MyActor|CheckifBlocked _returnvalue (Utilities|Struct|MakeIntVector (+ _x (.X (Utilities|Struct|BreakIntVector (Variables|BattleCharacteristics|GetPosition)))) (+ _y (.Y (Utilities|Struct|BreakIntVector (Variables|BattleCharacteristics|GetPosition))))))
    (Class|MyActor|SetCellIsOccupied _returnvalue (.x (Variables|BattleCharacteristics|GetPosition)) (.y (Variables|BattleCharacteristics|GetPosition)))
    (bind _output_get (Variables|BattleCharacteristics|SetPosition (Utilities|Struct|MakeIntVector (+ _x (.X (Utilities|Struct|BreakIntVector (Variables|BattleCharacteristics|GetPosition)))) (+ _y (.Y (Utilities|Struct|BreakIntVector (Variables|BattleCharacteristics|GetPosition)))))))
    (Class|MyActor|SetCellIsOccupied _returnvalue (.x _output_get) (.y _output_get) 2)
    (CallFunction|StartMove)
    (Math|Integer|DecrementInt (Variables|BattleCharacteristics|GetNumber%20Of%20Remaining%20Substeps)
      (:%20%20
        (return true)))
    (else
      (return false))))

(fn TryPickUp
  (bind _position (Variables|BattleCharacteristics|GetPosition))
  (bind (_x _y) (Utilities|Struct|BreakIntVector _position))
  (Actor|GetActorOfClass "/Game/Blueprints/Turn-Based.Turn-Based_C")
  (bind _outactors (Actor|GetAllActorsOfClass "/Game/Blueprints/PickUp.PickUp_C"))
  (bind _array_element (Utilities|Array|ForEachLoopwithBreak _outactors)
    (:LoopBody
      (if (and (== (.X (Utilities|Struct|BreakIntVector (Variables|/Game/Blueprints/PickUp.PickUp_C|GetPosition _array_element))) _x) (== (.Y (Utilities|Struct|BreakIntVector (Variables|/Game/Blueprints/PickUp.PickUp_C|GetPosition _array_element))) _y))
        (Default|PickUp _array_element)
        (return true)
        (else
          (return false))))))

(fn ReceiveDamageBase
  (params (Damage :type Integer))
  (bind _basedefense (Variables|BattleCharacteristics|GetbaseDefense))
  (bind _returnvalue (- Damage _basedefense))
  (if (> _returnvalue 0)
    (bind _output_get (Variables|BattleCharacteristics|SetHP (- (Variables|BattleCharacteristics|GetHP) _returnvalue)))
    (if (<= _output_get 0)
      (return true _returnvalue)
      (else
        (return false _returnvalue)))
    (else
      (return false 0))))

(fn TryAttack
  (params (Where :type Int%20Vector%20Structure%20%28by%20ref%29))
  (bind (_x _y) (Utilities|Struct|BreakIntVector Where))
  (bind _position (Variables|BattleCharacteristics|GetPosition))
  (bind (_x_2 _y_2) (Utilities|Struct|BreakIntVector _position))
  (Actor|GetActorOfClass "/Game/Blueprints/Turn-Based.Turn-Based_C")
  (bind _outactors (Actor|GetAllActorsOfClass "Creaturemy_C"))
  (bind _array_element (Utilities|Array|ForEachLoopwithBreak _outactors)
    (:LoopBody
      (if (and (== (.X (Utilities|Struct|BreakIntVector (Variables|Creaturemy_C|GetPosition _array_element))) (+ _x _x_2)) (== (.Y (Utilities|Struct|BreakIntVector (Variables|Creaturemy_C|GetPosition _array_element))) (+ _y _y_2)))
        (Development|PrintString "Attacking!")
        (Variables|BattleCharacteristics|SetIs%20in%20combat true)
        (CallFunction|ReceiveDamage _array_element (Variables|BattleCharacteristics|GetbaseAttack) 2)
        (Math|Integer|DecrementInt (Variables|BattleCharacteristics|GetNumber%20Of%20Remaining%20Substeps)
          (:%20%20
            (return true)))))
    (:Completed
      (return false))))

(fn Die
  (bind _position (Variables|BattleCharacteristics|GetPosition))
  (bind (_x _y) (Utilities|Struct|BreakIntVector _position))
  (bind _returnvalue (Actor|GetActorOfClass "/Script/Prototype.MyActor"))
  (Class|MyActor|SetCellIsOccupied _returnvalue _x _y)
  (Actor|DestroyActor))

(fn Heal
  (bind _maxhp (Variables|BattleCharacteristics|GetmaxHP))
  (if (<= (+ 0 (Variables|BattleCharacteristics|GetHP)) _maxhp)
    (Variables|BattleCharacteristics|SetHP (+ 0 (Variables|BattleCharacteristics|GetHP)))
    (else
      (Variables|BattleCharacteristics|SetHP _maxhp))))

(fn ReceiveDamage
  (params (Damage :type Integer) (effect :type Byte))
  (bind _returnvalue (Transformation|GetActorLocation))
  (Utilities|FlowControl|Sequence
    (:then_0
      (switch int (Math|Conversions|ToInteger(Byte) effect)
        (:1
          (Effects|SpawnEmitteratLocation "/Game/StarterContent/Particles/P_Explosion.P_Explosion" _returnvalue))
        (:2
          (Effects|SpawnEmitteratLocation "/Game/StarterContent/Particles/P_Sparks.P_Sparks" (+ _returnvalue "0, 0,200.000000")))))
    (:then_1
      (bind (_diddie _damagedid) (CallFunction|ReceiveDamageBase Damage))
      (Utilities|FlowControl|Sequence
        (:then_0
          (bind _returnvalue_2 (UserInterface|CreateWidget "/Game/Blueprints/UI/MyFloatingText.MyFloatingText_C" 0 (.ScreenPosition (Class|GameplayStatics|ProjectWorldtoScreen (Game|GetPlayerController 0) (+ (Transformation|GetActorLocation) "100.000000,0.000000,300.000000") false)) (Utilities|Text|ToText(Integer) (- 0 _damagedid))))
          (UserInterface|Viewport|AddtoViewport _returnvalue_2 0))
        (:then_1
          (if _diddie
            (CallFunction|Die)
            (return true)
            (else
              (return false))))))))

(fn UseItem)

(fn SetHealthWidget
  (bind _ashealth_info (Utilities|Casting|CastToHealthInfo (UserInterface|GetUserWidgetObject (Variables|Default|GetHealthWidget))))
  (Variables|/Game/Blueprints/UI/HealthInfo.HealthInfo_C|Setowner _ashealth_info self))