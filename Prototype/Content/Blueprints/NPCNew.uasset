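; Turn-based grid NPC that attacks, chases or wanders over a Game of Life board.
; Each turn NPCStep repeats until substeps or a safety counter run out, then TurnBased advances.
; It attacks or steps X-first toward the first Creature in Manhattan look range, otherwise wanders.
; Wander avoids cells about to be alive and also runs when its own cell will be; Navigation pathfinding is left disconnected.
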(event Custom|NPCStep
  (bind _number_of_remaining_substeps (Variables|Default|GetNumber%20Of%20Remaining%20Substeps))
  (bind _result (Math|Integer|DecrementInt (Variables|Default|Getcounter))
    (:%20%20
      (if (and (> _result 0) (> _number_of_remaining_substeps 0))
        (bind _issafe (CallFunction|CheckFloor))
        (if _issafe
          (bind (_isnear _canattack _where) (CallFunction|LookAround))
          (if _isnear
            (if _canattack
              (bind _success (CallFunction|TryAttack _where))
              (if _success
                (Utilities|FlowControl|Delay 0.8 :!label _label))
              (else
                (if (> (.X (Utilities|Struct|BreakIntVector _where)) 0)
                  (Variables|Default|SetTo%20Move (Utilities|Struct|MakeIntVector 1 0))
                  (elif (< (.X (Utilities|Struct|BreakIntVector _where)) 0)
                    (Variables|Default|SetTo%20Move (Utilities|Struct|MakeIntVector -1 0))
                    (elif (> (.Y (Utilities|Struct|BreakIntVector _where)) 0)
                      (Variables|Default|SetTo%20Move (Utilities|Struct|MakeIntVector 0 1))
                      (elif (< (.Y (Utilities|Struct|BreakIntVector _where)) 0)
                        (Variables|Default|SetTo%20Move (Utilities|Struct|MakeIntVector 0 -1))))))
                (CallFunction|TryMove (Variables|Default|GetTo%20Move))
                (goto _label)))
            (else
              (CallFunction|Wander :!label _label_2)
              (goto _label)))
          (else
            (goto _label_2)))
        (if (> _number_of_remaining_substeps 0)
          (CallFunction|NPCStep)
          (else
            (CallFunction|EndTurn)))
        (else
          (CallFunction|EndTurn))))))

(event Custom|EndTurn
  (Variables|Default|SetActive false)
  (Variables|Default|SetNumber%20Of%20Remaining%20Substeps 0)
  (bind _returnvalue (Actor|GetActorOfClass "/Game/Blueprints/Turn-Based.Turn-Based_C"))
  (Default|NextTurn _returnvalue))

(event Collision|EventActorBeginOverlap
  (params (OtherActor :type Actor%20Object%20Reference)))

(event EventBeginPlay
  (|CallParentFunction)
  (bind _returnvalue (Actor|GetActorOfClass "/Script/Prototype.MyActor"))
  (bind _returnvalue_2 (Actor|GetActorOfClass "/Script/Prototype.GoLUser")))

(event EventTick
  (params (DeltaSeconds :type Float%20%28single-precision%29)))

(event EventStartTurn
  (CallFunction|MessagetoList (Utilities|Text|ToText(String) (Variables|Default|GetName)) "'s turn" " ")
  (Variables|Default|SetNumber%20Of%20Remaining%20Substeps (Variables|Default|GetSpeed))
  (Variables|Default|SetActive true)
  (Variables|Default|Setcounter 10)
  (CallFunction|NPCStep))

(fn ConstructionScript)

(fn LookAround
  (bind _self self)
  (bind _position (Variables|Default|GetPosition _self))
  (bind (_x _y) (Utilities|Struct|BreakIntVector _position))
  (bind _outactors (Actor|GetAllActorsOfClass "/Game/Blueprints/Creature.Creature_C"))
  (bind _array_element (Utilities|Array|ForEachLoopwithBreak _outactors)
    (:LoopBody
      (if (and (<= (+ (Math|Integer|Absolute(Integer) (- (.X (Utilities|Struct|BreakIntVector (Variables|/Game/Blueprints/Creature.Creature_C|GetPosition _array_element))) _x)) (Math|Integer|Absolute(Integer) (- (.Y (Utilities|Struct|BreakIntVector (Variables|/Game/Blueprints/Creature.Creature_C|GetPosition _array_element))) _y))) (Variables|Default|GetlookRadius)) (> (+ (Math|Integer|Absolute(Integer) (- (.X (Utilities|Struct|BreakIntVector (Variables|/Game/Blueprints/Creature.Creature_C|GetPosition _array_element))) _x)) (Math|Integer|Absolute(Integer) (- (.Y (Utilities|Struct|BreakIntVector (Variables|/Game/Blueprints/Creature.Creature_C|GetPosition _array_element))) _y))) 0))
        (return (and (<= (+ (Math|Integer|Absolute(Integer) (- (.X (Utilities|Struct|BreakIntVector (Variables|/Game/Blueprints/Creature.Creature_C|GetPosition _array_element))) _x)) (Math|Integer|Absolute(Integer) (- (.Y (Utilities|Struct|BreakIntVector (Variables|/Game/Blueprints/Creature.Creature_C|GetPosition _array_element))) _y))) (Variables|Default|GetlookRadius)) (> (+ (Math|Integer|Absolute(Integer) (- (.X (Utilities|Struct|BreakIntVector (Variables|/Game/Blueprints/Creature.Creature_C|GetPosition _array_element))) _x)) (Math|Integer|Absolute(Integer) (- (.Y (Utilities|Struct|BreakIntVector (Variables|/Game/Blueprints/Creature.Creature_C|GetPosition _array_element))) _y))) 0)) (and (<= (+ (Math|Integer|Absolute(Integer) (- (.X (Utilities|Struct|BreakIntVector (Variables|/Game/Blueprints/Creature.Creature_C|GetPosition _array_element))) _x)) (Math|Integer|Absolute(Integer) (- (.Y (Utilities|Struct|BreakIntVector (Variables|/Game/Blueprints/Creature.Creature_C|GetPosition _array_element))) _y))) (Variables|Default|GetattackRadius)) (> (+ (Math|Integer|Absolute(Integer) (- (.X (Utilities|Struct|BreakIntVector (Variables|/Game/Blueprints/Creature.Creature_C|GetPosition _array_element))) _x)) (Math|Integer|Absolute(Integer) (- (.Y (Utilities|Struct|BreakIntVector (Variables|/Game/Blueprints/Creature.Creature_C|GetPosition _array_element))) _y))) 0)) (Utilities|Struct|MakeIntVector (- (.X (Utilities|Struct|BreakIntVector (Variables|/Game/Blueprints/Creature.Creature_C|GetPosition _array_element))) _x) (- (.Y (Utilities|Struct|BreakIntVector (Variables|/Game/Blueprints/Creature.Creature_C|GetPosition _array_element))) _y)))))
    (:Completed
      (return false false ""))))

(fn Wander
  (bind _returnvalue (Math|Random|RandomInteger 3))
  (bind _position (Variables|Default|GetPosition))
  (bind (_x _y) (Utilities|Struct|BreakIntVector _position))
  (bind _returnvalue_2 (Actor|GetActorOfClass "/Script/Prototype.GoLUser"))
  (Utilities|FlowControl|ForLoopwithBreak 0 8
    (:LoopBody
      (if (Class|GoLUser|WillbeAlive _returnvalue_2 (+ _x (.X (Utilities|Struct|BreakIntVector (Variables|Default|GetTo%20Move)))) (+ _y (.Y (Utilities|Struct|BreakIntVector (Variables|Default|GetTo%20Move)))))
        _
        (else
          (bind _success (CallFunction|TryMove (Variables|Default|GetTo%20Move)))
          (if _success
            (return)
            (else
              _))))
      (if (!= (.X (Utilities|Struct|BreakIntVector (Variables|Default|GetTo%20Move))) 0)
        (switch int _returnvalue
          (:Default
            (Variables|Default|SetTo%20Move (Utilities|Struct|MakeIntVector (* (.X (Utilities|Struct|BreakIntVector (Variables|Default|GetTo%20Move))) -1) 0)))
          (:0
            (Variables|Default|SetTo%20Move (Utilities|Struct|MakeIntVector 0 -1)))
          (:1
            (Variables|Default|SetTo%20Move (Utilities|Struct|MakeIntVector 0 1))))
        (else
          (switch int _returnvalue
            (:Default
              (Variables|Default|SetTo%20Move (Utilities|Struct|MakeIntVector 0 (* (.Y (Utilities|Struct|BreakIntVector (Variables|Default|GetTo%20Move))) -1))))
            (:0
              (Variables|Default|SetTo%20Move (Utilities|Struct|MakeIntVector 1 0)))
            (:1
              (Variables|Default|SetTo%20Move (Utilities|Struct|MakeIntVector -1 0)))))))
    (:Completed
      (Math|Integer|DecrementInt (Variables|Default|GetNumber%20Of%20Remaining%20Substeps)
        (:%20%20
          (return))))))

(fn CheckFloor
  (bind _self self)
  (bind _position (Variables|Default|GetPosition _self))
  (bind (_x _y) (Utilities|Struct|BreakIntVector _position))
  (bind _returnvalue (Actor|GetActorOfClass "/Script/Prototype.GoLUser"))
  (if (Class|GoLUser|WillbeAlive _returnvalue _x _y)
    (return false)
    (else
      (return true))))