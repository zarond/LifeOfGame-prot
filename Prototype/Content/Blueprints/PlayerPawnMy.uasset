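; Player pawn for a turn-based grid game with procedurally sized levels, moving in four directions within a per-turn substep budget based on Speed.
; Direction inputs share one TryMove path that picks up items or falls back to attacking when blocked, while Enter passes the turn to TurnBased.
; Navigation and NavButtons refresh as substeps change.
; Reaching the finish or pressing N enlarges the GameInstance's level dimensions and reloads the level; death reloads it unchanged.
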(event Custom|Attack
  (params (NewParam :type Int%20Vector%20Structure))
  ;[1 1 1] Обработка input событий
  (if (and (Variables|Default|GetActive) (> (Variables|Default|GetNumber%20Of%20Remaining%20Substeps) 0))
    (CallFunction|TryAttack NewParam)
    (CallFunction|SetUpNavigation (Variables|Default|GetNumber%20Of%20Remaining%20Substeps) 3)
    (else
      (Development|PrintString "Number of remaining substeps is zero. Press 'Enter' to continue."))))

(event Custom|UP
  (bind _position (Variables|Default|GetPosition))
  (bind (_x _y) (Utilities|Struct|BreakIntVector _position))
  ;[1 1 1] Обработка input событий
  (if (and (Variables|Default|GetActive) (> (Variables|Default|GetNumber%20Of%20Remaining%20Substeps) 0))
    (Variables|Default|SetTo%20Move (Utilities|Struct|MakeIntVector 1 0))
    (bind _success (CallFunction|TryMove (Variables|Default|GetTo%20Move)))
    (if _success
      (if (and (== _x (.X (Utilities|Struct|BreakIntVector (Class|MyActor|GetFinishPosition (stale EventBeginPlay _returnvalue))))) (== _y (.Y (Utilities|Struct|BreakIntVector (Class|MyActor|GetFinishPosition (stale EventBeginPlay _returnvalue))))))
        ;[1 1 1] check if finished level
        (bind _returnvalue (Game|GetCurrentLevelName true))
        (bind _asglobal (Utilities|Casting|CastToGlobal (Game|GetGameInstance)))
        (Variables|/Game/Blueprints/Global.Global_C|SetGHeight _asglobal (+ (Variables|/Game/Blueprints/Global.Global_C|GetGHeight _asglobal) 10))
        (Variables|/Game/Blueprints/Global.Global_C|SetGWidth _asglobal (+ (Variables|/Game/Blueprints/Global.Global_C|GetGWidth _asglobal) 10))
        (Game|OpenLevel(byName) (Utilities|String|StringToName _returnvalue))
        (else
          (CallFunction|TryPickUp)))
      (else
        (CallFunction|TryAttack (Variables|Default|GetTo%20Move))
        (CallFunction|SetUpNavigation (Variables|Default|GetNumber%20Of%20Remaining%20Substeps) 3)))
    (else
      (Development|PrintString "Number of remaining substeps is zero. Press 'Enter' to continue."))))

(event Custom|DOWN
  (bind _position (Variables|Default|GetPosition))
  (bind (_x _y) (Utilities|Struct|BreakIntVector _position))
  ;[1 1 1] Обработка input событий
  (if (and (Variables|Default|GetActive) (> (Variables|Default|GetNumber%20Of%20Remaining%20Substeps) 0))
    (Variables|Default|SetTo%20Move (Utilities|Struct|MakeIntVector -1 0))
    (bind _success (CallFunction|TryMove (Variables|Default|GetTo%20Move)))
    (if _success
      (if (and (== _x (.X (Utilities|Struct|BreakIntVector (Class|MyActor|GetFinishPosition (stale EventBeginPlay _returnvalue))))) (== _y (.Y (Utilities|Struct|BreakIntVector (Class|MyActor|GetFinishPosition (stale EventBeginPlay _returnvalue))))))
        ;[1 1 1] check if finished level
        (bind _returnvalue (Game|GetCurrentLevelName true))
        (bind _asglobal (Utilities|Casting|CastToGlobal (Game|GetGameInstance)))
        (Variables|/Game/Blueprints/Global.Global_C|SetGHeight _asglobal (+ (Variables|/Game/Blueprints/Global.Global_C|GetGHeight _asglobal) 10))
        (Variables|/Game/Blueprints/Global.Global_C|SetGWidth _asglobal (+ (Variables|/Game/Blueprints/Global.Global_C|GetGWidth _asglobal) 10))
        (Game|OpenLevel(byName) (Utilities|String|StringToName _returnvalue))
        (else
          (CallFunction|TryPickUp)))
      (else
        (CallFunction|TryAttack (Variables|Default|GetTo%20Move))
        (CallFunction|SetUpNavigation (Variables|Default|GetNumber%20Of%20Remaining%20Substeps) 3)))
    (else
      (Development|PrintString "Number of remaining substeps is zero. Press 'Enter' to continue."))))

(event Custom|RIGHT
  (bind _position (Variables|Default|GetPosition))
  (bind (_x _y) (Utilities|Struct|BreakIntVector _position))
  ;[1 1 1] Обработка input событий
  (if (and (Variables|Default|GetActive) (> (Variables|Default|GetNumber%20Of%20Remaining%20Substeps) 0))
    (Variables|Default|SetTo%20Move (Utilities|Struct|MakeIntVector 0 1))
    (bind _success (CallFunction|TryMove (Variables|Default|GetTo%20Move)))
    (if _success
      (if (and (== _x (.X (Utilities|Struct|BreakIntVector (Class|MyActor|GetFinishPosition (stale EventBeginPlay _returnvalue))))) (== _y (.Y (Utilities|Struct|BreakIntVector (Class|MyActor|GetFinishPosition (stale EventBeginPlay _returnvalue))))))
        ;[1 1 1] check if finished level
        (bind _returnvalue (Game|GetCurrentLevelName true))
        (bind _asglobal (Utilities|Casting|CastToGlobal (Game|GetGameInstance)))
        (Variables|/Game/Blueprints/Global.Global_C|SetGHeight _asglobal (+ (Variables|/Game/Blueprints/Global.Global_C|GetGHeight _asglobal) 10))
        (Variables|/Game/Blueprints/Global.Global_C|SetGWidth _asglobal (+ (Variables|/Game/Blueprints/Global.Global_C|GetGWidth _asglobal) 10))
        (Game|OpenLevel(byName) (Utilities|String|StringToName _returnvalue))
        (else
          (CallFunction|TryPickUp)))
      (else
        (CallFunction|TryAttack (Variables|Default|GetTo%20Move))
        (CallFunction|SetUpNavigation (Variables|Default|GetNumber%20Of%20Remaining%20Substeps) 3)))
    (else
      (Development|PrintString "Number of remaining substeps is zero. Press 'Enter' to continue."))))

(event Custom|LEFT
  (bind _position (Variables|Default|GetPosition))
  (bind (_x _y) (Utilities|Struct|BreakIntVector _position))
  ;[1 1 1] Обработка input событий
  (if (and (Variables|Default|GetActive) (> (Variables|Default|GetNumber%20Of%20Remaining%20Substeps) 0))
    (Variables|Default|SetTo%20Move (Utilities|Struct|MakeIntVector 0 -1))
    (bind _success (CallFunction|TryMove (Variables|Default|GetTo%20Move)))
    (if _success
      (if (and (== _x (.X (Utilities|Struct|BreakIntVector (Class|MyActor|GetFinishPosition (stale EventBeginPlay _returnvalue))))) (== _y (.Y (Utilities|Struct|BreakIntVector (Class|MyActor|GetFinishPosition (stale EventBeginPlay _returnvalue))))))
        ;[1 1 1] check if finished level
        (bind _returnvalue (Game|GetCurrentLevelName true))
        (bind _asglobal (Utilities|Casting|CastToGlobal (Game|GetGameInstance)))
        (Variables|/Game/Blueprints/Global.Global_C|SetGHeight _asglobal (+ (Variables|/Game/Blueprints/Global.Global_C|GetGHeight _asglobal) 10))
        (Variables|/Game/Blueprints/Global.Global_C|SetGWidth _asglobal (+ (Variables|/Game/Blueprints/Global.Global_C|GetGWidth _asglobal) 10))
        (Game|OpenLevel(byName) (Utilities|String|StringToName _returnvalue))
        (else
          (CallFunction|TryPickUp)))
      (else
        (CallFunction|TryAttack (Variables|Default|GetTo%20Move))
        (CallFunction|SetUpNavigation (Variables|Default|GetNumber%20Of%20Remaining%20Substeps) 3)))
    (else
      (Development|PrintString "Number of remaining substeps is zero. Press 'Enter' to continue."))))

(event Custom|EndTurn
  (Variables|Default|SetActive false)
  (bind _returnvalue (Actor|GetActorOfClass "/Game/Blueprints/Turn-Based.Turn-Based_C"))
  (Default|NextTurn _returnvalue))

(event EventDie
  (CallFunction|DieandReset))

(event EventBeginPlay
  (bind _returnvalue (Actor|GetActorOfClass "/Script/Prototype.MyActor"))
  (bind _returnvalue_2 (Actor|GetActorOfClass "/Script/Prototype.GoLUser"))
  (Class|NavigationComponent|SetGlobalActor (Variables|Default|GetNavigation) _returnvalue _returnvalue_2))

(event EventFinishMove
  (Variables|Default|SetMoving false)
  (Development|PrintString "Goodbye")
  (CallFunction|SetUpNavigation (Variables|Default|GetNumber%20Of%20Remaining%20Substeps) 3))

(event EventStartTurn
  (Variables|Default|SetNumber%20Of%20Remaining%20Substeps (Variables|Default|GetSpeed))
  (Variables|Default|SetActive true)
  (CallFunction|SetUpNavigation (Variables|Default|GetNumber%20Of%20Remaining%20Substeps) 3)
  (CallFunction|TryPickUp))

(event EventStartMove
  (Variables|Default|SetMoving true)
  (Development|PrintString "Hello 2"))

(event Input|ActionEvents|InputActionEnter
  (params (Key :type Key%20Structure))
  (:Pressed
    (if (Variables|Default|GetActive)
      (bind _output_get (Variables|Default|SetNumber%20Of%20Remaining%20Substeps 0))
      (CallFunction|SetUpNavigation _output_get 3)
      (CallFunction|EndTurn))))

(event Input|ActionEvents|InputActionMoveUp
  (params (Key :type Key%20Structure))
  (:Pressed
    (CallFunction|UP)))

(event Input|ActionEvents|InputActionMoveDown
  (params (Key :type Key%20Structure))
  (:Pressed
    (CallFunction|DOWN)))

(event Input|ActionEvents|InputActionMoveLeft
  (params (Key :type Key%20Structure))
  (:Pressed
    (CallFunction|LEFT)))

(event Input|ActionEvents|InputActionMoveRight
  (params (Key :type Key%20Structure))
  (:Pressed
    (CallFunction|RIGHT)))

(event Input|KeyboardEvents|N
  (params (Key :type Key%20Structure))
  ;[1 1 1] check if finished level
  (:Pressed
    (bind _returnvalue (Game|GetCurrentLevelName true))
    (bind _asglobal (Utilities|Casting|CastToGlobal (Game|GetGameInstance)))
    (Variables|/Game/Blueprints/Global.Global_C|SetGHeight _asglobal (+ (Variables|/Game/Blueprints/Global.Global_C|GetGHeight _asglobal) 10))
    (Variables|/Game/Blueprints/Global.Global_C|SetGWidth _asglobal (+ (Variables|/Game/Blueprints/Global.Global_C|GetGWidth _asglobal) 10))
    (Game|OpenLevel(byName) (Utilities|String|StringToName _returnvalue))))

(fn ConstructionScript)

(fn ReceiveDamage0
  (params (Damage :type Integer))
  (bind _diddie (CallFunction|ReceiveDamageBase Damage))
  (if _diddie
    (CallFunction|DieandReset)
    (return true)
    (else
      (return false))))

(fn DieandReset
  (bind _returnvalue (Game|GetCurrentLevelName true))
  (Game|OpenLevel(byName) (Utilities|String|StringToName _returnvalue)))

(fn SetUpNavigation
  (params (newRadius :type Integer) (Energy :type Integer))
  (bind _position (Variables|Default|GetPosition))
  (bind (_x _y) (Utilities|Struct|BreakIntVector _position))
  (Class|NavigationComponent|SetUp (Variables|Default|GetNavigation) _x _y newRadius Energy)
  (bind _returnvalue (Actor|GetActorOfClass "/Game/Blueprints/PROCEDUAL.Procedual_C"))
  (Class|NavButtonsComponent|UpdateButtons (Variables|Default|GetNavButtons) (Math|Conversions|ToFloat(Integer) (Variables|/Game/Blueprints/PROCEDUAL.Procedual_C|GetPolygon%20Size _returnvalue))))