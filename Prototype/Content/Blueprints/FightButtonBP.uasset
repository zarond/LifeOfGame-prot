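; FightButtonBP is a clickable grid-cell target that makes the player pawn attack toward its X/Y position.
; Hovering swaps the Sphere to a lamp material and sets a crosshair cursor; leaving restores the walnut material and default cursor, and destruction also resets the cursor.
; On click it prints its coordinates, casts the player pawn to PlayerPawn and calls Attack with the offset from the pawn's Position.
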(event EventBeginPlay)

(event Collision|EventActorBeginOverlap
  (params (OtherActor :type Actor%20Object%20Reference)))

(event EventTick
  (params (DeltaSeconds :type Float%20%28single-precision%29)))

(event MouseInput|EventActorBeginCursorOver
  (Rendering|Material|SetMaterial (Variables|Default|GetSphere) 0 "/Game/StarterContent/Props/Materials/M_Lamp.M_Lamp")
  (Variables|/Script/Engine.PlayerController|SetCurrentMouseCursor (Game|GetPlayerController 0) "Crosshairs"))

(event MouseInput|EventActorEndCursorOver
  (Rendering|Material|SetMaterial (Variables|Default|GetSphere) 0 "/Game/StarterContent/Materials/M_Wood_Walnut.M_Wood_Walnut")
  (Variables|/Script/Engine.PlayerController|SetCurrentMouseCursor (Game|GetPlayerController 0) "Default"))

(event MouseInput|EventActorOnClicked
  (params (ButtonPressed :type Key%20Structure :default "None"))
  (Development|PrintString (Utilities|String|Append (Utilities|String|Append (Utilities|String|Append (Utilities|String|ToString(Integer) (Variables|Default|Getx)) " ") (Utilities|String|ToString(Integer) (Variables|Default|Gety))) " ButtonPress") true false)
  (bind _asplayer_pawn (Utilities|Casting|CastToPlayerPawn (Game|Player|GetPlayerPawn 0)))
  (Default|Attack _asplayer_pawn (Utilities|Struct|MakeIntVector (- (Variables|Default|Getx) (.X (Utilities|Struct|BreakIntVector (Variables|/Game/Blueprints/Creature.Creature_C|GetPosition _asplayer_pawn)))) (- (Variables|Default|Gety) (.Y (Utilities|Struct|BreakIntVector (Variables|/Game/Blueprints/Creature.Creature_C|GetPosition _asplayer_pawn)))))))

(event EventDestroyed
  (Variables|/Script/Engine.PlayerController|SetCurrentMouseCursor (Game|GetPlayerController 0) "Default"))

(fn ConstructionScript)