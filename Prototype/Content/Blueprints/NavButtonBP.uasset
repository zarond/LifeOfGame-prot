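; NavButtonBP is a clickable navigation button actor with an Arrow component that highlights under the cursor.
; Cursor-over events swap the arrow's material to M_Lamp on hover and back to the stored Material variable when the cursor leaves.
; Clicking only prints the button's X and Y values with a "ButtonPress" suffix, with no navigation logic in this graph.
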(event EventBeginPlay)

(event Collision|EventActorBeginOverlap
  (params (OtherActor :type Actor%20Object%20Reference)))

(event EventTick
  (params (DeltaSeconds :type Float%20%28single-precision%29)))

(event MouseInput|EventActorBeginCursorOver
  (Rendering|Material|SetMaterial (Variables|Components|Getarrow) 0 "/Game/StarterContent/Props/Materials/M_Lamp.M_Lamp"))

(event MouseInput|EventActorEndCursorOver
  (Rendering|Material|SetMaterial (Variables|Components|Getarrow) 0 "/Game/Material.Material"))

(event MouseInput|EventActorOnClicked
  (params (ButtonPressed :type Key%20Structure :default "None"))
  (Development|PrintString (Utilities|String|Append (Utilities|String|Append (Utilities|String|Append (Utilities|String|ToString(Integer) (Variables|Default|Getx)) " ") (Utilities|String|ToString(Integer) (Variables|Default|Gety))) " ButtonPress") true false))

(fn ConstructionScript)