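; Turn manager Blueprint that runs an endless round-based turn order over player pawns, NPCNew actors and the GOLUserBP actor.
; SetUp builds that ordered list at BeginPlay, and each NextTurn call sends StartTurnMessage to the next valid entity, skipping invalid ones.
; Past the list's end, CleanUpAfterRound filters out invalid references and NextRound restarts the counters.
; A zero-length Delay precedes each turn, and the counter increments before the message is sent.
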(event Custom|Next%20Round
  (Math|Integer|IncrementInt (Variables|NewModel|GetRoundNumber)
    (:%20%20
      (Variables|NewModel|Setcounter 0)
      (Variables|NewModel|SetTurnNumber 0)
      (CallFunction|NextTurn))))

(event Custom|Next%20Turn
  (Utilities|FlowControl|Delay 0.0) ; без этого почему-то не работает
  (if (Utilities|Array|IsValidIndex (Variables|NewModel|GetPlayingEntities) (Variables|NewModel|Getcounter)) :!label _label
    (Utilities|IsValid (Utilities|Array|Get(acopy) (Variables|NewModel|GetPlayingEntities) (Variables|NewModel|Getcounter))
      (:Is%20Valid
        (Math|Integer|IncrementInt (Variables|NewModel|GetTurnNumber)
          (:%20%20
            ;[1 1 1] Один из 2х вариантов. Этот работает без Delay
            (Math|Integer|IncrementInt (Variables|NewModel|Getcounter)
              (:%20%20
                (Class|GameInterface|StartTurn(Message) (Utilities|Array|Get(acopy) (Variables|NewModel|GetPlayingEntities) (- (Variables|NewModel|Getcounter) 1))))))))
      (:Is%20Not%20Valid
        (Math|Integer|IncrementInt (Variables|NewModel|Getcounter)
          (:%20%20
            (Development|PrintString "Not Valid")
            (goto _label)))))
    (else
      (CallFunction|CleanUpAfterRound)
      (CallFunction|NextRound))))

(event EventBeginPlay
  (CallFunction|SetUp)
  (CallFunction|NextRound))

(fn ConstructionScript)

(fn SetUp
  ;[1 1 1] Создания массива всех играющих сущностей в порядке - все игроки, npc, GOL
  (Utilities|FlowControl|Sequence
    (:then_0
      (bind _returnvalue (Class|GameModeBase|GetNumPlayers))
      (for _index (range 0 (- _returnvalue 1))
        (Utilities|Array|Add (Variables|NewModel|GetPlayingEntities) (Game|Player|GetPlayerPawn _index))))
    (:then_1
      (bind _outactors (Actor|GetAllActorsOfClass "/Game/Blueprints/NPCNew.NPCNew_C"))
      (Utilities|Array|AppendArray (Variables|NewModel|GetPlayingEntities) _outactors))
    (:then_2
      (bind _returnvalue_2 (Actor|GetActorOfClass "/Game/Blueprints/GOLUserBP.GOLUserBP_C"))
      (Utilities|Array|Add (Variables|NewModel|GetPlayingEntities) _returnvalue_2))
    (:then_3
      (return))))

(fn CleanUpAfterRound
  ;[1 1 1] Избавляемся от пустых ссылок
  (for _array_element (Variables|NewModel|GetPlayingEntities)
    (Utilities|IsValid _array_element
      (:Is%20Valid
        (Utilities|Array|Add (LocalVariables|Gettmp) _array_element))))
  (Variables|NewModel|SetPlayingEntities (LocalVariables|Gettmp))
  (return))