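; Base NPC actor for a turn-based, grid-positioned game, with health, damage handling and death.
; It adds a behaviour component on BeginPlay, which EnemyTurn queries for move, attack and defence values, prints as debug output, then advances and resets substeps.
; Lethal damage, or a turn begun with negative HP, triggers Die, which frees the grid cell, leaves the TurnBased manager's NPC array and destroys the actor.
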(event EventBeginPlay
  (bind _returnvalue (AddComponent|AddBehaviour))
  (Variables|Default|SetBehaviourClass _returnvalue))

(event Collision|EventActorBeginOverlap
  (params (OtherActor :type Actor%20Object%20Reference)))

(event EventTick
  (params (DeltaSeconds :type Float%20%28single-precision%29)))

(fn ConstructionScript)

(fn EnemyTurn
  (bind _behaviourclass (Variables|Default|GetBehaviourClass))
  (if (>= (Variables|Default|GetHP) 0)
    (if (Variables|Default|GetisInBattle)
      (Development|PrintString "In battle!"))
    (Utilities|FlowControl|Sequence
      (:then_0
        (bind _returnvalue (Class|Behaviour|GetMove _behaviourclass)))
      (:then_1
        (bind _returnvalue_2 (Class|Behaviour|GetAttack _behaviourclass)))
      (:then_2
        (bind _returnvalue_3 (Class|Behaviour|GetDefence _behaviourclass)))
      (:then_3
        (Development|PrintString "EnemyAction")
        (bind _returnvalue_4 (Class|Behaviour|GetSubsteps _behaviourclass))
        (Development|PrintString (Utilities|String|ToString(Integer) _returnvalue_4))
        (Development|PrintString (Utilities|String|Append (LocalVariables|GetMoveWord) (Utilities|String|ToString(Integer) _returnvalue)))
        (Development|PrintString (Utilities|String|Append (LocalVariables|GetAttackWord) (Utilities|String|ToString(Integer) _returnvalue_2)))
        (Development|PrintString (Utilities|String|Append (LocalVariables|GetDefenceWord) (Utilities|String|ToString(Integer) _returnvalue_3)))
        (Class|Behaviour|NextStep _behaviourclass)
        (Class|Behaviour|SetSubsteps _behaviourclass 3)
        (bind _returnvalue_5 (Class|Behaviour|GetSubsteps _behaviourclass))
        (Development|PrintString (Utilities|String|ToString(Integer) _returnvalue_5))))
    (else
      (CallFunction|Die))))

(fn TakeВamage
  (params (Damage :type Integer))
  (if (<= (- (Variables|Default|GetHP) Damage) 0)
    (CallFunction|Die)
    (else
      (Variables|Default|SetHP (- (Variables|Default|GetHP) Damage)))))

(fn Die
  (bind _position (Variables|Default|GetPosition))
  (bind (_x _y) (Utilities|Struct|BreakIntVector _position))
  (bind _returnvalue (Actor|GetActorOfClass "/Game/Blueprints/Turn-Based.Turn-Based_C"))
  (bind _returnvalue_2 (Actor|GetActorOfClass "/Script/Prototype.MyActor"))
  (Class|MyActor|SetCellIsOccupied _returnvalue_2 _x _y)
  (Utilities|Array|RemoveIndex (Variables|/Game/Blueprints/Turn-Based.Turn-Based_C|GetArrayOfNPCs _returnvalue) (Utilities|Array|FindItem (Variables|/Game/Blueprints/Turn-Based.Turn-Based_C|GetArrayOfNPCs _returnvalue) self))
  (Actor|DestroyActor))